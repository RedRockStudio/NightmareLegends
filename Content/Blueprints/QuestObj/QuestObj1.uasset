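; QuestObj1 is a carryable quest item whose mesh, material, rotation and hint effect offset are configurable per instance.
; When taken, it disables collision and follows the player's QLoc every tick, updating hand state and widget.
; On release, it is pushed along camera forward with physics, then frozen after a retriggerable delay.
; Hard impacts send the first AiEnemy1 to the noise location, while softer ones only play a quieter sound.
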(event `self.ReceiveTick`
  (params (DeltaSeconds :type "Float (single-precision)"))
  ;[1 0.125 0.125] Event Tick
  (`|ExecutionSequence`
    (:`then_0`
      (`self.EventTickForTransformUpdate`))))

(event `EventTickForTransformUpdate`
  ;[1 1 1] Take
  (if (`self.Taken`)
    (bind _asfirst_person_character (cast `/Game/FirstPersonBP/Blueprints/FirstPersonCharacter` (`GameplayStatics.GetPlayerPawn` 0) :!label _label))
    (`SceneComponent.K2_SetWorldTransform` (`self.QuestObj`) (`SceneComponent.K2_GetComponentToWorld` (`/Game/FirstPersonBP/Blueprints/FirstPersonCharacter.QLoc` _asfirst_person_character)) false false)))

(event `questObjTake`
  ;[1 1 1] Take
  (`GameplayStatics.PlaySound2D` (`self.TakeQuestObjSnd`) 1.0 1.0 0.0 null null)
  (set `self.Taken` true)
  (`PrimitiveComponent.SetCollisionEnabled` (`self.QuestObj`) "NoCollision")
  (bind _asfirst_person_character (cast `/Game/FirstPersonBP/Blueprints/FirstPersonCharacter` (`GameplayStatics.GetPlayerPawn` 0)))
  (set `/Game/FirstPersonBP/Blueprints/FirstPersonCharacter.IsHandEmpty?` false _asfirst_person_character)
  (`|ExecutionSequence`
    (:`then_0`
      (goto _label))
    (:`then_1`
      (bind _asfirst_person_character_2 (cast `/Game/FirstPersonBP/Blueprints/FirstPersonCharacter` (`GameplayStatics.GetPlayerPawn` 0)))
      (`/Game/Widgets/MainWidget.ShowGrabButton` (`/Game/FirstPersonBP/Blueprints/FirstPersonCharacter.MainWidget` _asfirst_person_character_2)))
    (:`then_2`
      (`GameplayStatics.PlaySound2D` null 1.0 1.0 0.0 null null))
    (:`then_3`
      (`SceneComponent.SetVisibility` (`self.HintFX`) false false))))

(event `questObjRelease`
  (bind _questobj (`self.QuestObj`))
  ;[1 1 1] Drop
  (`GameplayStatics.PlaySound2D` "/Game/Audio/SndFX/itemDrop.itemDrop" 1.0 1.0 0.0 null null)
  (set `self.Taken` false)
  (`SceneComponent.SetVisibility` (`self.HintFX`) true false)
  (`PrimitiveComponent.SetCollisionEnabled` (`self.QuestObj`) "QueryAndPhysics")
  (bind _asfirst_person_character (cast `/Game/FirstPersonBP/Blueprints/FirstPersonCharacter` (`GameplayStatics.GetPlayerPawn` 0)))
  (set `/Game/FirstPersonBP/Blueprints/FirstPersonCharacter.IsHandEmpty?` true _asfirst_person_character)
  (`PrimitiveComponent.SetSimulatePhysics` _questobj true)
  (`PrimitiveComponent.AddImpulse` _questobj (`KismetMathLibrary.GetForwardVector` (`SceneComponent.K2_GetComponentRotation` (`/Game/FirstPersonBP/Blueprints/FirstPersonCharacter.FirstPersonCamera` _asfirst_person_character))) "None" false)
  (bind _asfirst_person_character_2 (cast `/Game/FirstPersonBP/Blueprints/FirstPersonCharacter` (`GameplayStatics.GetPlayerPawn` 0)))
  (`/Game/Widgets/MainWidget.HideDropButton` (`/Game/FirstPersonBP/Blueprints/FirstPersonCharacter.MainWidget` _asfirst_person_character_2))
  (`KismetSystemLibrary.RetriggerableDelay` (`self.FreezeTimer`))
  (`PrimitiveComponent.SetSimulatePhysics` (`self.QuestObj`) false))

(event `self.QuestObj.OnComponentHit`
  (params (HitComponent :type "PrimitiveComponent Object Reference") (OtherActor :type "Actor Object Reference") (OtherComp :type "PrimitiveComponent Object Reference") (NormalImpulse :type "Vector Structure") (Hit :type "HitResult Structure (by ref)"))
  (bind _returnvalue (`KismetMathLibrary.VSize` NormalImpulse))
  ;[1 1 1] MakeNoise
  (if (> _returnvalue 1300.0)
    (bind _output_get (set `self.NoiseLastQObjLoc` Hit_Location))
    (`GameplayStatics.PlaySoundAtLocation` "/Game/Audio/SndFX/fall_Cue.fall_Cue" _output_get (struct) 0.85 1.0 0.0 null null null) ; SoundForEnemyHear
    (bind _outactors (`GameplayStatics.GetAllActorsOfClass` "/Game/Blueprints/AI1BP/AiEnemy1.AiEnemy1_C"))
    (bind _output (`|GetArrayItem` _outactors))
    (set `/Game/Blueprints/AI1BP/AiEnemy1.NoiseObjLoc` (`self.NoiseLastQObjLoc`) _output)
    (`/Game/Blueprints/AI1BP/AiEnemy1.GoToNoiseObjLocation` _output)
    (elif (> _returnvalue 150.0)
      (`GameplayStatics.PlaySoundAtLocation` (`self.FallingSnd`) _output_get (struct) 0.35 1.0 0.0 null null null) ; SoundForSilentFall
    )))

(fn `UserConstructionScript`
  (locals (NewLocalVar_0 :type "Float (double-precision)" :default 0.0))
  (bind _questobj (`self.QuestObj`))
  (`StaticMeshComponent.SetStaticMesh` _questobj (`self.CustomMesh`))
  (`SceneComponent.K2_AddRelativeRotation` _questobj (`self.RotationOffset`) false false)
  (`PrimitiveComponent.SetMaterial` _questobj 0 (`self.CustomMaterial`))
  (`SceneComponent.K2_AddRelativeLocation` (`self.HintFX`) (`self.AddHintOffsetLocation`) false false))