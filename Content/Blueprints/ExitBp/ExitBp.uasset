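; ExitBp is a level exit trigger that completes the level once the player has enough objectives and a key.
; When the first-person character overlaps its Box, it reads the Item and Key counters from FirstPersonGameMode.
; A sequence of checks either shows a main widget tip naming what is missing, with a locked-door sound, or sets LevelCompleted and calls LevelCompete on the character.
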(event `self.Box.OnComponentBeginOverlap`
  (params (OverlappedComponent :type "PrimitiveComponent Object Reference") (OtherActor :type "Actor Object Reference") (OtherComp :type "PrimitiveComponent Object Reference") (OtherBodyIndex :type Integer) (bFromSweep :type Boolean) (SweepResult :type "HitResult Structure (by ref)"))
  (cast `/Game/FirstPersonBP/Blueprints/FirstPersonCharacter` OtherActor)
  (bind _asfirst_person_game_mode (cast `/Game/FirstPersonBP/Blueprints/FirstPersonGameMode` (`GameplayStatics.GetGameMode`)))
  (`|ExecutionSequence`
    (:`then_0`
      (bind _item (`/Game/FirstPersonBP/Blueprints/FirstPersonGameMode.Item` _asfirst_person_game_mode))
      (bind _key (`/Game/FirstPersonBP/Blueprints/FirstPersonGameMode.Key` _asfirst_person_game_mode))
      ;[1 1 1] Tips
      (if (and (< _item 9.0) (< _key 1.0))
        (bind _asfirst_person_character (cast `/Game/FirstPersonBP/Blueprints/FirstPersonCharacter` (`GameplayStatics.GetPlayerPawn` 0)))
        (bind _mainwidget (`/Game/FirstPersonBP/Blueprints/FirstPersonCharacter.MainWidget` _asfirst_person_character))
        (set `/Game/Widgets/MainWidget.CurrTipName` "ObjsNKey" _mainwidget)
        (`/Game/Widgets/MainWidget.Tips` _mainwidget :!label _label)
        (`/Game/Widgets/MainWidget.Tips` (`/Game/FirstPersonBP/Blueprints/FirstPersonCharacter.MainWidget` (stale _asfirst_person_character_3)))
        (`/Game/Widgets/MainWidget.Tips` (`/Game/FirstPersonBP/Blueprints/FirstPersonCharacter.MainWidget` (stale _asfirst_person_character_2)))
        (`GameplayStatics.PlaySoundAtLocation` "/Game/Audio/SndFX/LockedDoor.LockedDoor" (`SceneComponent.K2_GetComponentLocation` (`self.Box`)) (struct) 1.0 1.0 0.0 null null null)))
    (:`then_1`
      (if (and (> _key 0.0) (<= _item 8.0))
        (bind _asfirst_person_character_2 (cast `/Game/FirstPersonBP/Blueprints/FirstPersonCharacter` (`GameplayStatics.GetPlayerPawn` 0)))
        (set `/Game/Widgets/MainWidget.CurrTipName` "Objs" (`/Game/FirstPersonBP/Blueprints/FirstPersonCharacter.MainWidget` _asfirst_person_character_2))
        (goto _label)))
    (:`then_2`
      (if (and (== _key 0.0) (>= _item 9.0))
        (bind _asfirst_person_character_3 (cast `/Game/FirstPersonBP/Blueprints/FirstPersonCharacter` (`GameplayStatics.GetPlayerPawn` 0)))
        (set `/Game/Widgets/MainWidget.CurrTipName` "Key" (`/Game/FirstPersonBP/Blueprints/FirstPersonCharacter.MainWidget` _asfirst_person_character_3))
        (goto _label)))
    (:`then_3`
      ;[1 1 1] LevelComplete
      (if (and (>= (`/Game/FirstPersonBP/Blueprints/FirstPersonGameMode.Key` _asfirst_person_game_mode) 1.0) (>= (`/Game/FirstPersonBP/Blueprints/FirstPersonGameMode.Item` _asfirst_person_game_mode) 9.0))
        (bind _asfirst_person_character_4 (cast `/Game/FirstPersonBP/Blueprints/FirstPersonCharacter` (`GameplayStatics.GetPlayerPawn` 0)))
        (set `/Game/FirstPersonBP/Blueprints/FirstPersonCharacter.LevelCompleted` true _asfirst_person_character_4)
        (`/Game/FirstPersonBP/Blueprints/FirstPersonCharacter.LevelCompete` _asfirst_person_character_4)))))

(fn `UserConstructionScript`)