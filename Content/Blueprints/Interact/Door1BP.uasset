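; Interactive door actor that swings open once when something overlaps either of its two trigger boxes, LBox or RBox.
; Each box plays its own timeline to drive the door mesh's relative yaw, alongside an attenuated opening sound at the mesh's location.
; The DoorFloat boolean gates both triggers and is cleared during timeline updates, with no reset or closing logic in the graph.
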(event `self.LBox.OnComponentBeginOverlap`
  (params (OverlappedComponent :type "PrimitiveComponent Object Reference") (OtherActor :type "Actor Object Reference") (OtherComp :type "PrimitiveComponent Object Reference") (OtherBodyIndex :type Integer) (bFromSweep :type Boolean) (SweepResult :type "HitResult Structure (by ref)"))
  (if (`self.DoorFloat`)
    (`|ExecutionSequence`
      (:`then_0`
        (bind (_direction _opendoorleft) (`Timeline|Timeline_0`)
          (:`Update`
            (`SceneComponent.K2_SetRelativeRotation` (`self.DoorMesh`) (`KismetMathLibrary.MakeRotator` 0.0 0.0 _opendoorleft) false false)
            (set `self.DoorFloat` false))))
      (:`then_1`
        (`GameplayStatics.PlaySoundAtLocation` "/Game/Audio/SndFX/OpenDoor1_Cue.OpenDoor1_Cue" (`SceneComponent.K2_GetComponentLocation` (`self.DoorMesh`)) (struct) 2.0 1.0 0.0 "/Game/Audio/SND_Attenuation1.SND_Attenuation1" null null)))))

(event `self.RBox.OnComponentBeginOverlap`
  (params (OverlappedComponent :type "PrimitiveComponent Object Reference") (OtherActor :type "Actor Object Reference") (OtherComp :type "PrimitiveComponent Object Reference") (OtherBodyIndex :type Integer) (bFromSweep :type Boolean) (SweepResult :type "HitResult Structure (by ref)"))
  (if (`self.DoorFloat`)
    (`|ExecutionSequence`
      (:`then_0`
        (bind (_direction _opendoorleft) (`Timeline|Timeline_1`)
          (:`Update`
            (`SceneComponent.K2_SetRelativeRotation` (`self.DoorMesh`) (`KismetMathLibrary.MakeRotator` 0.0 0.0 _opendoorleft) false false)
            (set `self.DoorFloat` false))))
      (:`then_1`
        (`GameplayStatics.PlaySoundAtLocation` "/Game/Audio/SndFX/OpenDoor1_Cue.OpenDoor1_Cue" (`SceneComponent.K2_GetComponentLocation` (`self.DoorMesh`)) (struct) 2.0 1.0 0.0 "/Game/Audio/SND_Attenuation1.SND_Attenuation1" null null)))))

(fn `UserConstructionScript`)