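; BP_TableSlider is an interactable table with a sliding part that may hold a battery pickup.
; On BeginPlay a one-in-four roll destroys the child actor, labelled as the battery, so its presence varies.
; TableSliderOpenClose, called from outside, uses a FlipFlop to ease the slider open or shut with a sliding sound.
; A box trigger sets the FirstPersonCharacter's AtTumba flag while the character overlaps it.
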(event `self.ReceiveBeginPlay`
  ;[0.4375 0.3001 0.08567] EventBeginPlay
  (if (== (`KismetMathLibrary.RandomIntegerInRange` 0 3) 0)
    (`ActorComponent.K2_DestroyComponent` (`self.ChildActor`)) ; DestroyBattery
  ))

(event `TableSliderOpenClose`
  (bind _tableslider (`self.TableSlider`))
  (bind _returnvalue (`SceneComponent.K2_GetComponentLocation` (`self.Table`)))
  ;[0.09543 1 0.47] Slider
  (`/Engine/EditorBlueprintResources/StandardMacros.FlipFlop`
    (:`A`
      (`GameplayStatics.PlaySoundAtLocation` "/Game/Audio/SndFX/PicSliding.PicSliding" _returnvalue (struct) 1.0 1.0 0.0 "/Game/Audio/SND_Attenuation1.SND_Attenuation1" null null)
      (`KismetSystemLibrary.MoveComponentTo` _tableslider (0.0 35.0 79.0) (struct) true true 0.65))
    (:`B`
      (`GameplayStatics.PlaySoundAtLocation` "/Game/Audio/SndFX/PicSliding.PicSliding" _returnvalue (struct) 1.0 1.0 0.0 "/Game/Audio/SND_Attenuation1.SND_Attenuation1" null null)
      (`KismetSystemLibrary.MoveComponentTo` _tableslider (0.0 7.5 79.0) (struct) true true 0.65))))

(event `self.Box.OnComponentBeginOverlap`
  (params (OverlappedComponent :type "PrimitiveComponent Object Reference") (OtherActor :type "Actor Object Reference") (OtherComp :type "PrimitiveComponent Object Reference") (OtherBodyIndex :type Integer) (bFromSweep :type Boolean) (SweepResult :type "HitResult Structure (by ref)"))
  ;[0.2031 0.1764 0.03326] AtTable?
  (bind _asfirst_person_character (cast `/Game/FirstPersonBP/Blueprints/FirstPersonCharacter` OtherActor))
  (set `/Game/FirstPersonBP/Blueprints/FirstPersonCharacter.AtTumba?` true _asfirst_person_character))

(event `self.Box.OnComponentEndOverlap`
  (params (OverlappedComponent :type "PrimitiveComponent Object Reference") (OtherActor :type "Actor Object Reference") (OtherComp :type "PrimitiveComponent Object Reference") (OtherBodyIndex :type Integer))
  ;[0.2031 0.1764 0.03326] AtTable?
  (bind _asfirst_person_character (cast `/Game/FirstPersonBP/Blueprints/FirstPersonCharacter` OtherActor))
  (set `/Game/FirstPersonBP/Blueprints/FirstPersonCharacter.AtTumba?` false _asfirst_person_character))

(fn `UserConstructionScript`)