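; Interactive cabinet (tumba) that opens and closes either a hinged door or a sliding drawer, with sound.
; TumbaComponentActivation picks the part via DoorOrSlider, and a FlipFlop on each alternates open and close through eased MoveComponentTo moves.
; A box overlap sets or clears AtTumba on the FirstPersonCharacter.
; On BeginPlay it has a one-in-four chance to destroy its child actor, noted as a battery.
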(event `self.ReceiveBeginPlay`
  ;[0.4375 0.3001 0.08567] EventBeginPlay
  (if (== (`KismetMathLibrary.RandomIntegerInRange` 0 3) 0)
    (`ActorComponent.K2_DestroyComponent` (`self.ChildActor`)) ; DestroyBattery
  ))

(event `TumbaComponentActivation`
  ;[1 1 1] ChooseEvent
  (if (`self.DoorOrSlider`)
    (`self.TumbaSliderOpenClose`)
    (else
      (`self.TumbaDoorOpenClose`))))

(event `TumbaDoorOpenClose`
  (bind _tumbadoor (`self.TumbaDoor`))
  (bind _returnvalue (`SceneComponent.K2_GetComponentLocation` (`self.Tumba`)))
  ;[0.4896 0.1195 0.1635] Door
  (`/Engine/EditorBlueprintResources/StandardMacros.FlipFlop`
    (:`A`
      (`GameplayStatics.PlaySoundAtLocation` "/Game/Audio/SndFX/OpenDoor1_Cue.OpenDoor1_Cue" _returnvalue (struct) 1.0 1.0 0.0 "/Game/Audio/SND_Attenuation1.SND_Attenuation1" null null)
      (`KismetSystemLibrary.MoveComponentTo` _tumbadoor (23.0 19.0 36.0) (struct :`Yaw` -90.0) true true 0.65))
    (:`B`
      (`GameplayStatics.PlaySoundAtLocation` "/Game/Audio/SndFX/OpenDoor1_Cue.OpenDoor1_Cue" _returnvalue (struct) 1.0 1.0 0.0 "/Game/Audio/SND_Attenuation1.SND_Attenuation1" null null)
      (`KismetSystemLibrary.MoveComponentTo` _tumbadoor (23.0 19.0 36.0) (struct) true true 0.65))))

(event `self.Box.OnComponentBeginOverlap`
  (params (OverlappedComponent :type "PrimitiveComponent Object Reference") (OtherActor :type "Actor Object Reference") (OtherComp :type "PrimitiveComponent Object Reference") (OtherBodyIndex :type Integer) (bFromSweep :type Boolean) (SweepResult :type "HitResult Structure (by ref)"))
  ;[0.2031 0.1764 0.03326] AtTumba?
  (bind _asfirst_person_character (cast `/Game/FirstPersonBP/Blueprints/FirstPersonCharacter` OtherActor))
  (set `/Game/FirstPersonBP/Blueprints/FirstPersonCharacter.AtTumba?` true _asfirst_person_character))

(event `self.Box.OnComponentEndOverlap`
  (params (OverlappedComponent :type "PrimitiveComponent Object Reference") (OtherActor :type "Actor Object Reference") (OtherComp :type "PrimitiveComponent Object Reference") (OtherBodyIndex :type Integer))
  ;[0.2031 0.1764 0.03326] AtTumba?
  (bind _asfirst_person_character (cast `/Game/FirstPersonBP/Blueprints/FirstPersonCharacter` OtherActor))
  (set `/Game/FirstPersonBP/Blueprints/FirstPersonCharacter.AtTumba?` false _asfirst_person_character))

(event `TumbaSliderOpenClose`
  (bind _tumbaslider (`self.TumbaSlider`))
  (bind _returnvalue (`SceneComponent.K2_GetComponentLocation` (`self.Tumba`)))
  ;[0.09543 1 0.47] Slider
  (`/Engine/EditorBlueprintResources/StandardMacros.FlipFlop`
    (:`A`
      (`GameplayStatics.PlaySoundAtLocation` "/Game/Audio/SndFX/PicSliding.PicSliding" _returnvalue (struct) 1.0 1.0 0.0 "/Game/Audio/SND_Attenuation1.SND_Attenuation1" null null)
      (`KismetSystemLibrary.MoveComponentTo` _tumbaslider (0.0 16.0 71.0) (struct) true true 0.65))
    (:`B`
      (`GameplayStatics.PlaySoundAtLocation` "/Game/Audio/SndFX/PicSliding.PicSliding" _returnvalue (struct) 1.0 1.0 0.0 "/Game/Audio/SND_Attenuation1.SND_Attenuation1" null null)
      (`KismetSystemLibrary.MoveComponentTo` _tumbaslider (0.0 -3.7 71.0) (struct) true true 0.65))))

(fn `UserConstructionScript`)