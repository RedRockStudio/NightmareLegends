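; BP_MCabinDoor is a morgue cabinet door that serves as a one-shot scare when the player walks near it.
; On BeginPlay a coin flip either arms the trigger or sets the door to a fixed rotation, leaving it inactive.
; If armed, the first FirstPersonCharacter overlap with the box disarms it, swings the door's yaw through a timeline and plays scary and metal door 2D sounds.
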(event `self.ReceiveBeginPlay`
  ;[1 1 1] Active
  (if (== (`KismetMathLibrary.RandomIntegerInRange` 0 1) 0)
    (set `self.Activate` true)
    (else
      (`SceneComponent.K2_SetWorldRotation` (`self.MorgCabinsDoor`) (struct :`Yaw` 90.0) false false))))

(event `self.Box.OnComponentBeginOverlap`
  (params (OverlappedComponent :type "PrimitiveComponent Object Reference") (OtherActor :type "Actor Object Reference") (OtherComp :type "PrimitiveComponent Object Reference") (OtherBodyIndex :type Integer) (bFromSweep :type Boolean) (SweepResult :type "HitResult Structure (by ref)"))
  (cast `/Game/FirstPersonBP/Blueprints/FirstPersonCharacter` OtherActor)
  (if (`self.Activate`)
    (set `self.Activate` false)
    (`|ExecutionSequence`
      (:`then_0`
        (bind (_direction _opendoorleft) (`Timeline|Timeline_0`)
          (:`Update`
            (`SceneComponent.K2_SetRelativeRotation` (`self.MorgCabinsDoor`) (`KismetMathLibrary.MakeRotator` 0.0 0.0 _opendoorleft) false false))))
      (:`then_1`
        (`GameplayStatics.PlaySound2D` "/Game/Audio/SndFX/ScaryFX1_Cue.ScaryFX1_Cue" 1.0 1.0 0.0 null null)
        (`GameplayStatics.PlaySound2D` "/Game/Audio/SndFX/MetalDoor_Cue.MetalDoor_Cue" 1.0 1.0 0.0 null null)))))

(fn `UserConstructionScript`)