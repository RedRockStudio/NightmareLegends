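; BP_CreakFloor is a trigger volume that makes a floorboard creak and lures the enemy AI to it.
; When FirstPersonCharacter enters the Box, a one-in-four roll, gated by an Overlapped flag cleared on exit, plays the creak sound at the actor's root.
; It then passes that location to the first AiEnemy1 found via GetAllActorsOfClass and calls its GoToNoiseObjLocation.
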(event `self.Box.OnComponentBeginOverlap`
  (params (OverlappedComponent :type "PrimitiveComponent Object Reference") (OtherActor :type "Actor Object Reference") (OtherComp :type "PrimitiveComponent Object Reference") (OtherBodyIndex :type Integer) (bFromSweep :type Boolean) (SweepResult :type "HitResult Structure (by ref)"))
  (bind _returnvalue (`SceneComponent.K2_GetComponentLocation` (`self.DefaultSceneRoot`)))
  (cast `/Game/FirstPersonBP/Blueprints/FirstPersonCharacter` OtherActor)
  (if (and (== (`KismetMathLibrary.RandomIntegerInRange` 0 3) 1) (not (`self.Overlapped`)))
    (`GameplayStatics.PlaySoundAtLocation` "/Game/Audio/SndFX/floorWoodCreak_Cue.floorWoodCreak_Cue" _returnvalue (struct) 1.0 1.0 0.0 null null null)
    (set `self.CreakNoiseLoc` _returnvalue)
    (set `self.Overlapped` true)
    (bind _outactors (`GameplayStatics.GetAllActorsOfClass` "/Game/Blueprints/AI1BP/AiEnemy1.AiEnemy1_C"))
    (bind _asai_enemy_1 (cast `/Game/Blueprints/AI1BP/AiEnemy1` (`|GetArrayItem` _outactors)))
    (set `/Game/Blueprints/AI1BP/AiEnemy1.NoiseObjLoc` (`self.CreakNoiseLoc`) _asai_enemy_1)
    (`/Game/Blueprints/AI1BP/AiEnemy1.GoToNoiseObjLocation` _asai_enemy_1)))

(event `self.Box.OnComponentEndOverlap`
  (params (OverlappedComponent :type "PrimitiveComponent Object Reference") (OtherActor :type "Actor Object Reference") (OtherComp :type "PrimitiveComponent Object Reference") (OtherBodyIndex :type Integer))
  (cast `/Game/FirstPersonBP/Blueprints/FirstPersonCharacter` OtherActor)
  (set `self.Overlapped` false))

(fn `UserConstructionScript`)