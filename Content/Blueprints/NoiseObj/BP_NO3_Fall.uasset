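; BP_NO3_Fall is a noise prop that falls when the player walks into its trigger box and draws the enemy to the sound.
; The first overlap enables physics on the mesh and applies a random horizontal impulse.
; Hard hits play a falling sound and send the first AiEnemy1 found to the impact location.
; Hits also start a delay that switches physics off.
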(event `self.Box.OnComponentBeginOverlap`
  (params (OverlappedComponent :type "PrimitiveComponent Object Reference") (OtherActor :type "Actor Object Reference") (OtherComp :type "PrimitiveComponent Object Reference") (OtherBodyIndex :type Integer) (bFromSweep :type Boolean) (SweepResult :type "HitResult Structure (by ref)"))
  (bind _staticmesh (`self.StaticMesh`))
  (cast `/Game/FirstPersonBP/Blueprints/FirstPersonCharacter` OtherActor)
  (if (not (`self.Activated`))
    (`PrimitiveComponent.SetSimulatePhysics` _staticmesh true)
    (`PrimitiveComponent.AddImpulse` _staticmesh (`KismetMathLibrary.MakeVector` (`KismetMathLibrary.RandomFloatInRange` -200.0 200.0) (`KismetMathLibrary.RandomFloatInRange` -200.0 200.0)) "None" false)
    (set `self.Activated` true)))

(event `self.StaticMesh.OnComponentHit`
  (params (HitComponent :type "PrimitiveComponent Object Reference") (OtherActor :type "Actor Object Reference") (OtherComp :type "PrimitiveComponent Object Reference") (NormalImpulse :type "Vector Structure") (Hit :type "HitResult Structure (by ref)"))
  (`|ExecutionSequence`
    (:`then_0`
      (`KismetSystemLibrary.Delay` 4.0)
      (`PrimitiveComponent.SetSimulatePhysics` (`self.StaticMesh`) false))
    (:`then_1`
      (if (> (`KismetMathLibrary.VSize` NormalImpulse) 150.0)
        (bind _output_get (set `self.NoiseLastLoc` Hit_Location))
        (`GameplayStatics.PlaySoundAtLocation` (`self.FallingSnd`) _output_get (struct) 0.8 1.0 0.0 null null null)
        (bind _outactors (`GameplayStatics.GetAllActorsOfClass` "/Game/Blueprints/AI1BP/AiEnemy1.AiEnemy1_C"))
        (bind _asai_enemy_1 (cast `/Game/Blueprints/AI1BP/AiEnemy1` (`|GetArrayItem` _outactors)))
        (set `/Game/Blueprints/AI1BP/AiEnemy1.NoiseObjLoc` (`self.NoiseLastLoc`) _asai_enemy_1)
        (`/Game/Blueprints/AI1BP/AiEnemy1.GoToNoiseObjLocation` _asai_enemy_1)))))

(fn `UserConstructionScript`)