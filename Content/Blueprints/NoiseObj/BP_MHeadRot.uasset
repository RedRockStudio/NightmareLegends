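; BP_MHeadRot is a one-shot scare prop whose mannequin head turns when the player walks into its trigger box.
; On BeginPlay a random roll arms it about half the time.
; When armed, an overlap by FirstPersonCharacter disarms it, plays a 2D scare sound and runs a timeline that drives the head's relative yaw.
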(event `self.ReceiveBeginPlay`
  ;[1 1 1] Active
  (if (== (`KismetMathLibrary.RandomIntegerInRange` 0 1) 0)
    (set `self.Activate` true)))

(event `self.Box.OnComponentBeginOverlap`
  (params (OverlappedComponent :type "PrimitiveComponent Object Reference") (OtherActor :type "Actor Object Reference") (OtherComp :type "PrimitiveComponent Object Reference") (OtherBodyIndex :type Integer) (bFromSweep :type Boolean) (SweepResult :type "HitResult Structure (by ref)"))
  (cast `/Game/FirstPersonBP/Blueprints/FirstPersonCharacter` OtherActor)
  (if (`self.Activate`)
    (set `self.Activate` false)
    (`GameplayStatics.PlaySound2D` "/Game/Audio/SndFX/ScaryFX1_Cue.ScaryFX1_Cue" 1.0 1.0 0.0 null null)
    (bind (_direction _opendoorleft) (`Timeline|Timeline_0` :!via `PlayFromStart`)
      (:`Update`
        (`SceneComponent.K2_SetRelativeRotation` (`self.MannHead`) (`KismetMathLibrary.MakeRotator` 0.0 0.0 _opendoorleft) false false)))))

(fn `UserConstructionScript`)