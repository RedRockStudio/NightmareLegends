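; BP_TVNoise is a one-shot trigger that makes a TV static disturbance when the player walks into it.
; On BeginPlay it randomly arms itself with a 50% chance.
; When a FirstPersonCharacter overlaps its box while armed, it disarms, briefly shows DecalPlane and plays an attenuated static sound at the plane's location.
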(event `self.ReceiveBeginPlay`
  ;[1 1 1] Active
  (if (== (`KismetMathLibrary.RandomIntegerInRange` 0 1) 0)
    (set `self.Activate` true)))

(event `self.Box.OnComponentBeginOverlap`
  (params (OverlappedComponent :type "PrimitiveComponent Object Reference") (OtherActor :type "Actor Object Reference") (OtherComp :type "PrimitiveComponent Object Reference") (OtherBodyIndex :type Integer) (bFromSweep :type Boolean) (SweepResult :type "HitResult Structure (by ref)"))
  (bind _decalplane (`self.DecalPlane`))
  (cast `/Game/FirstPersonBP/Blueprints/FirstPersonCharacter` OtherActor)
  (if (`self.Activate`)
    (set `self.Activate` false)
    (`|ExecutionSequence`
      (:`then_0`
        (`SceneComponent.SetVisibility` _decalplane true false)
        (`KismetSystemLibrary.Delay` 9.0)
        (`SceneComponent.SetVisibility` _decalplane false false))
      (:`then_1`
        (`GameplayStatics.PlaySoundAtLocation` "/Game/Audio/SndFX/TVStatic_Cue.TVStatic_Cue" (`SceneComponent.K2_GetComponentLocation` (`self.DecalPlane`)) (struct) 1.2 1.0 0.0 "/Game/Audio/SND_Attenuation2.SND_Attenuation2" null null)))))

(fn `UserConstructionScript`)