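; Balloon scare prop that has a 50/50 chance of being active when play begins.
; An active balloon loops its animation, while an inactive one is hidden.
; When the first-person character overlaps its box, an active balloon disarms, hides and plays 2D pop, scary effect and evil laugh sounds together, so it fires only once.
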(event `self.ReceiveBeginPlay`
  (bind _velballoon (`self.velBalloon`))
  ;[1 1 1] Active
  (if (== (`KismetMathLibrary.RandomIntegerInRange` 0 1) 0)
    (set `self.Activate` true)
    (`SkeletalMeshComponent.PlayAnimation` _velballoon "/Game/Geometry/Props/Anims/velBalloon_Anim.velBalloon_Anim" true)
    (else
      (`SceneComponent.SetVisibility` _velballoon false false))))

(event `self.Box.OnComponentBeginOverlap`
  (params (OverlappedComponent :type "PrimitiveComponent Object Reference") (OtherActor :type "Actor Object Reference") (OtherComp :type "PrimitiveComponent Object Reference") (OtherBodyIndex :type Integer) (bFromSweep :type Boolean) (SweepResult :type "HitResult Structure (by ref)"))
  (cast `/Game/FirstPersonBP/Blueprints/FirstPersonCharacter` OtherActor)
  (if (`self.Activate`)
    (set `self.Activate` false)
    (`|ExecutionSequence`
      (:`then_0`
        (`SceneComponent.SetVisibility` (`self.velBalloon`) false false))
      (:`then_1`
        (`GameplayStatics.PlaySound2D` "/Game/Audio/SndFX/BalloonPop_Cue.BalloonPop_Cue" 1.0 1.0 0.0 null null)
        (`GameplayStatics.PlaySound2D` "/Game/Audio/SndFX/ScaryFX1_Cue.ScaryFX1_Cue" 1.0 1.0 0.0 null null)
        (`GameplayStatics.PlaySound2D` "/Game/Audio/SndFX/EvilLaugh_Cue.EvilLaugh_Cue" 1.0 1.0 0.0 null null)))))

(fn `UserConstructionScript`)