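; BP_ScreamerFaceActivator is a trigger actor that springs a screamer-face scare on the player.
; On BeginPlay a coin flip decides whether this instance is armed.
; When the FirstPersonCharacter overlaps its Box while armed, it calls ScreamerFaceEvent on the character's MainWidget and disarms, so the scare fires only once.
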(event `self.ReceiveBeginPlay`
  ;[1 1 1] Switcher
  (if (== (`KismetMathLibrary.RandomIntegerInRange` 0 1) 0)
    (set `self.activate` true)))

(event `self.Box.OnComponentBeginOverlap`
  (params (OverlappedComponent :type "PrimitiveComponent Object Reference") (OtherActor :type "Actor Object Reference") (OtherComp :type "PrimitiveComponent Object Reference") (OtherBodyIndex :type Integer) (bFromSweep :type Boolean) (SweepResult :type "HitResult Structure (by ref)"))
  (bind _asfirst_person_character (cast `/Game/FirstPersonBP/Blueprints/FirstPersonCharacter` OtherActor))
  (if (`self.activate`)
    (`/Game/Widgets/MainWidget.ScreamerFaceEvent` (`/Game/FirstPersonBP/Blueprints/FirstPersonCharacter.MainWidget` _asfirst_person_character))
    (set `self.activate` false)))

(fn `UserConstructionScript`)