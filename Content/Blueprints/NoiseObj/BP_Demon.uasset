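; BP_Demon is a one-shot jump scare that has a 50% chance to be armed at BeginPlay; otherwise it hides its DemonScreamer mesh.
; When the FirstPersonCharacter overlaps its Box while armed, it disarms and waits briefly.
; It then shows the demon playing a non-looping scream animation alongside two 2D scare sounds, and hides it again after a short delay.
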(event `self.ReceiveBeginPlay`
  ;[1 1 1] Active
  (if (== (`KismetMathLibrary.RandomIntegerInRange` 0 1) 0)
    (set `self.Activate` true)
    (else
      (`SceneComponent.SetVisibility` (`self.DemonScreamer`) false false))))

(event `self.Box.OnComponentBeginOverlap`
  (params (OverlappedComponent :type "PrimitiveComponent Object Reference") (OtherActor :type "Actor Object Reference") (OtherComp :type "PrimitiveComponent Object Reference") (OtherBodyIndex :type Integer) (bFromSweep :type Boolean) (SweepResult :type "HitResult Structure (by ref)"))
  (bind _demonscreamer (`self.DemonScreamer`))
  (cast `/Game/FirstPersonBP/Blueprints/FirstPersonCharacter` OtherActor)
  (if (`self.Activate`)
    (set `self.Activate` false)
    (`KismetSystemLibrary.Delay` 0.75)
    (`|ExecutionSequence`
      (:`then_0`
        (`SceneComponent.SetVisibility` _demonscreamer true false)
        (`SkeletalMeshComponent.PlayAnimation` _demonscreamer "/Game/Geometry/char/Screamers/DemonScreamer_Anim.DemonScreamer_Anim" false)
        (`KismetSystemLibrary.Delay` 1.6)
        (`SceneComponent.SetVisibility` (`self.DemonScreamer`) false false))
      (:`then_1`
        (`GameplayStatics.PlaySound2D` "/Game/Audio/SndFX/DemonScream_Cue.DemonScream_Cue" 1.0 1.0 0.0 null null)
        (`GameplayStatics.PlaySound2D` "/Game/Audio/SndFX/ScaryFX1_Cue.ScaryFX1_Cue" 1.0 1.0 0.0 null null)))))

(fn `UserConstructionScript`)