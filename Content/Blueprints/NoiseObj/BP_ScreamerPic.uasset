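; BP_ScreamerPic is a one-shot jump-scare picture that has a coin-flip chance of being armed at BeginPlay.
; When armed, the first FirstPersonCharacter overlap with its Box disarms it and fires the scare.
; The scare briefly reveals PicFace with its animation, hides it after a delay, and plays scream and scary-effect sounds in 2D.
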(event `self.ReceiveBeginPlay`
  ;[1 1 1] Active
  (if (== (`KismetMathLibrary.RandomIntegerInRange` 0 1) 0)
    (set `self.Activate` true)))

(event `self.Box.OnComponentBeginOverlap`
  (params (OverlappedComponent :type "PrimitiveComponent Object Reference") (OtherActor :type "Actor Object Reference") (OtherComp :type "PrimitiveComponent Object Reference") (OtherBodyIndex :type Integer) (bFromSweep :type Boolean) (SweepResult :type "HitResult Structure (by ref)"))
  (bind _picface (`self.PicFace`))
  (cast `/Game/FirstPersonBP/Blueprints/FirstPersonCharacter` OtherActor)
  (if (`self.Activate`)
    (set `self.Activate` false)
    (`|ExecutionSequence`
      (:`then_0`
        (`SceneComponent.SetVisibility` _picface true false)
        (`SkeletalMeshComponent.PlayAnimation` _picface "/Game/Geometry/Props/Anims/PicFace_Anim.PicFace_Anim" false)
        (`KismetSystemLibrary.Delay` 2.333)
        (`SceneComponent.SetVisibility` _picface false false))
      (:`then_1`
        (`GameplayStatics.PlaySound2D` "/Game/Audio/SndFX/PicScream_Cue.PicScream_Cue" 1.0 1.0 0.0 null null)
        (`GameplayStatics.PlaySound2D` "/Game/Audio/SndFX/ScaryFX1_Cue.ScaryFX1_Cue" 1.0 1.0 0.0 null null)))))

(fn `UserConstructionScript`)