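; Main menu GameMode that shows the mouse cursor, caches player save data and then calls CallMMStart.
; SaveGameMM loads the NLSave slot into MM variables for progress, coins, achievements, diary and settings, or creates and saves a new MysterySaveGame if none exists.
; ReSaveGameMM writes only music volume, sound volume and camera sensitivity back to the slot, then re-runs SaveGameMM to refresh the cache.
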(event `self.ReceiveBeginPlay`
  (set `PlayerController.bShowMouseCursor` true (`GameplayStatics.GetPlayerController` 0))
  (`self.SaveGameMM`)
  (`self.MM_Start`))

(event `SaveGameMM`
  (bind _savegameconnection (`self.SaveGameConnection`))
  ;[1 1 1] SaveGameMM
  (bind _returnvalue (`GameplayStatics.DoesSaveGameExist` "NLSave"))
  (if _returnvalue
    (bind _returnvalue_2 (`GameplayStatics.LoadGameFromSlot` "NLSave"))
    (set `self.SaveGameConnection` _returnvalue_2)
    (bind _asmystery_save_game (cast `/Game/Blueprints/SaveGame/MysterySaveGame` _savegameconnection))
    (set `self.MM_BestTime` (`/Game/Blueprints/SaveGame/MysterySaveGame.BestTime` _asmystery_save_game))
    (set `self.MM_PlayerCoins` (`/Game/Blueprints/SaveGame/MysterySaveGame.PlayerCoins` _asmystery_save_game))
    (set `self.MM_Map1Ach` (`/Game/Blueprints/SaveGame/MysterySaveGame.Map1Achievements` _asmystery_save_game))
    (set `self.MM_Map1Diary` (`/Game/Blueprints/SaveGame/MysterySaveGame.Map1Diary` _asmystery_save_game))
    (set `self.MM_LevelUnlocked` (`/Game/Blueprints/SaveGame/MysterySaveGame.LevelUnlocked` _asmystery_save_game))
    (set `self.MM_MusVol` (`/Game/Blueprints/SaveGame/MysterySaveGame.MusVol` _asmystery_save_game))
    (set `self.MM_SndVol` (`/Game/Blueprints/SaveGame/MysterySaveGame.SndVol` _asmystery_save_game))
    (set `self.MM_CanSens` (`/Game/Blueprints/SaveGame/MysterySaveGame.CamSensivity` _asmystery_save_game))
    (else
      (bind _returnvalue_3 (`GameplayStatics.CreateSaveGameObject` "/Game/Blueprints/SaveGame/MysterySaveGame.MysterySaveGame_C"))
      (set `self.SaveGameConnection` _returnvalue_3)
      (bind _asmystery_save_game_2 (cast `/Game/Blueprints/SaveGame/MysterySaveGame` _savegameconnection))
      (`GameplayStatics.SaveGameToSlot` _asmystery_save_game_2 "NLSave"))))

(event `ReSaveGameMM`
  ;[0.1006 0.3594 0.224] ReSaveGame
  (bind _asmystery_save_game (cast `/Game/Blueprints/SaveGame/MysterySaveGame` (`self.SaveGameConnection`)))
  (set `/Game/Blueprints/SaveGame/MysterySaveGame.CamSensivity` (`self.MM_CanSens`) _asmystery_save_game)
  (set `/Game/Blueprints/SaveGame/MysterySaveGame.MusVol` (`self.MM_MusVol`) _asmystery_save_game)
  (set `/Game/Blueprints/SaveGame/MysterySaveGame.SndVol` (`self.MM_SndVol`) _asmystery_save_game)
  (`GameplayStatics.SaveGameToSlot` _asmystery_save_game "NLSave")
  (`self.SaveGameMM`) ; ReCacheDataFromSaveGame
)

(fn `UserConstructionScript`)