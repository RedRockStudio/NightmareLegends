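; Monster enemy AI that hunts and kills the player, with speeds set by game difficulty and removal in Practice.
; Event-driven AIMoveTo calls and state flags run random nine-point patrols with voice lines, noise investigation, and PawnSensing-triggered chases.
; Closet-hidden players are tracked to their last navmesh location; visible ones via line trace.
; Standard and under-bed kill events play animations, death widget and fade, with Tick-fed gates zooming the camera.
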(event `self.ReceiveBeginPlay`
  ;[1 1 1] Difficulty
  (`|ExecutionSequence`
    (:`then_0`
      (bind _asnl_game_instance (cast `/Game/Blueprints/GameInstance/NL_GameInstance` (`GameplayStatics.GetGameInstance`)))
      (if (== (`/Game/Blueprints/GameInstance/NL_GameInstance.DifficultyMode` _asnl_game_instance) "Practice")
        (`self.K2_DestroyActor`)))
    (:`then_1`
      (bind _asnl_game_instance_2 (cast `/Game/Blueprints/GameInstance/NL_GameInstance` (`GameplayStatics.GetGameInstance`)))
      (if (== (`/Game/Blueprints/GameInstance/NL_GameInstance.DifficultyMode` _asnl_game_instance_2) "Normal")
        (set `self.ChaseRunSpeed` 225.0)
        (set `self.PatrolSpeed` 50.0)
        (set `self.NoiseRunSpeed` 175.0)))
    (:`then_2`
      (bind _asnl_game_instance_3 (cast `/Game/Blueprints/GameInstance/NL_GameInstance` (`GameplayStatics.GetGameInstance`)))
      (if (== (`/Game/Blueprints/GameInstance/NL_GameInstance.DifficultyMode` _asnl_game_instance_3) "Hard")
        (set `self.ChaseRunSpeed` 350.0)
        (set `self.PatrolSpeed` 150.0)
        (set `self.NoiseRunSpeed` 250.0)))))

(event `AIStarter`
  ;[1 1 1] BeginPlay
  (`self.Patrol`)
  (bind _asfirst_person_character (cast `/Game/FirstPersonBP/Blueprints/FirstPersonCharacter` (`GameplayStatics.GetPlayerPawn` 0)))
  (set `self.player` _asfirst_person_character))

(event `GoToNoiseObjLocation`
  ;[1 0.9152 0.2937] GoToNoiseObject
  (set `CharacterMovementComponent.MaxWalkSpeed` (`self.NoiseRunSpeed`) (`self.CharacterMovement`))
  (if (not (and (`self.GoToNoise`) (`self.CanSee`) (`self.TargetOnOff`)))
    (set `self.GoToNoiseObj` true)
    (`|AIMoveTo` self (`self.NoiseObjLoc`) null 50.0
      (:`OnSuccess`
        _)
      (:`OnFail`
        _))
    (`KismetSystemLibrary.Delay` (`KismetMathLibrary.RandomFloatInRange` 3.0 6.0))
    (set `self.GoToNoiseObj` false)
    (`self.Patrol`)))

(event `self.ReceiveTick`
  (params (DeltaSeconds :type "Float (single-precision)"))
  ;[0.09131 0.2396 0.125] EventTick
  (`self.EventTickUnderBed` DeltaSeconds)
  (`self.EventTickDeath` DeltaSeconds))

(event `Patrol`
  ;[0.04341 0.08705 0.5365] Patrol
  (`self.SaySmthg`)
  (if (`self.TargetOnOff`)
    _
    (elif (not (`self.GoToNoise`))
      (bind _asmonster_1animation (cast `/Game/Geometry/char/Enemy1/Monster1Animation` (`SkeletalMeshComponent.GetAnimInstance` (`self.Mesh`))))
      (set `CharacterMovementComponent.MaxWalkSpeed` (`self.PatrolSpeed`) (`self.CharacterMovement`))
      (set `/Game/Geometry/char/Enemy1/Monster1Animation.HeadRotationFloat` 0.0 _asmonster_1animation)
      (set `/Game/Geometry/char/Enemy1/Monster1Animation.HeadRotationFloat2` 0.0 _asmonster_1animation)
      (set `/Game/Geometry/char/Enemy1/Monster1Animation.HeadRotationFloat3` 0.0 _asmonster_1animation)
      (set `/Game/Geometry/char/Enemy1/Monster1Animation.NewVar_0` (0.0 0.0 0.0) _asmonster_1animation)
      (switch `int` (`KismetMathLibrary.RandomIntegerInRange` 0 8)
        (:`0`
          (`|AIMoveTo` self (0.0 0.0 0.0) (`self.TargetPont4`)
            (:`OnSuccess`
              (`KismetSystemLibrary.Delay` 1.0))))
        (:`1`
          (`|AIMoveTo` self (0.0 0.0 0.0) (`self.TargetPont5`)
            (:`OnSuccess`
              (`KismetSystemLibrary.Delay` 1.0))))
        (:`2`
          (`|AIMoveTo` self (0.0 0.0 0.0) (`self.TargetPont6`)
            (:`OnSuccess`
              (`KismetSystemLibrary.Delay` 1.0))))
        (:`3`
          (`|AIMoveTo` self (0.0 0.0 0.0) (`self.TargetPont7`)
            (:`OnSuccess`
              (`KismetSystemLibrary.Delay` 1.0))))
        (:`4`
          (`|AIMoveTo` self (0.0 0.0 0.0) (`self.TargetPont8`)
            (:`OnSuccess`
              (`KismetSystemLibrary.Delay` 1.0))))
        (:`5`
          (`|AIMoveTo` self (0.0 0.0 0.0) (`self.TargetPont9`)
            (:`OnSuccess`
              (`KismetSystemLibrary.Delay` 1.0))))
        (:`6`
          (`|AIMoveTo` self (0.0 0.0 0.0) (`self.TargetPont1`)
            (:`OnSuccess`
              (`KismetSystemLibrary.Delay` 1.0))))
        (:`7`
          (`|AIMoveTo` self (0.0 0.0 0.0) (`self.TargetPont2`)
            (:`OnSuccess`
              (`KismetSystemLibrary.Delay` 1.0))))
        (:`8`
          (`|AIMoveTo` self (0.0 0.0 0.0) (`self.TargetPont3`)
            (:`OnSuccess`
              (`KismetSystemLibrary.Delay` 1.0)))))
      (`self.Patrol`))))

(event `self.PawnSensing.OnHearNoise`
  (params (Instigator :type "Pawn Object Reference") (Location :type "Vector Structure (by ref)") (Volume :type "Float (single-precision)"))
  ;[1 1 1] PawnHearNoise
  (set `CharacterMovementComponent.MaxWalkSpeed` (`self.NoiseRunSpeed`) (`self.CharacterMovement`))
  (if (`self.Can hear`)
    (set `self.TargetOnOff` true)
    (set `self.GoToNoise` true)
    (bind _asfirst_person_character (cast `/Game/FirstPersonBP/Blueprints/FirstPersonCharacter` (`GameplayStatics.GetPlayerCharacter` 0)))
    (`|AIMoveTo` self (`self.K2_GetActorLocation` _asfirst_person_character) null
      (:`OnSuccess`
        _)
      (:`OnFail`
        _))
    (`KismetSystemLibrary.Delay` (`KismetMathLibrary.RandomFloatInRange` 3.0 6.0))
    (set `self.GoToNoise` false)
    (set `self.TargetOnOff` false)
    (`self.Patrol`)))

(event `self.PawnSensing.OnSeePawn`
  (params (Pawn :type "Pawn Object Reference"))
  (bind _player (`self.player`))
  ;[0.4115 0.1059 0.3904] OnSeePawn
  (if (not (or (`/Game/FirstPersonBP/Blueprints/FirstPersonCharacter.PlayerDied` _player) (`/Game/FirstPersonBP/Blueprints/FirstPersonCharacter.PlayerHiddenForSense` _player)))
    (set `self.TargetOnOff` true)
    (if (`/Game/FirstPersonBP/Blueprints/FirstPersonCharacter.IsPlayerHiddenCloset` _player)
      (`self.RunToLastPlayerLoc`)
      (else
        (`self.StandartChaseEvent`)))))

(event `AiWin`
  (bind _killanimarray (`self.KillAnimArray`))
  (bind (_returnvalue_roll _returnvalue_pitch _returnvalue_yaw) (`KismetMathLibrary.BreakRotator` (`KismetMathLibrary.FindLookAtRotation` (`self.K2_GetActorLocation`) (`self.K2_GetActorLocation` (`self.player`)))))
  ;[1 0.02604 0.02604] AiWin
  (`/Engine/EditorBlueprintResources/StandardMacros.DoOnce` false
    (:`Completed`
      (`|ExecutionSequence`
        (:`then_0`
          (`GameplayStatics.PlaySound2D` "/Game/Audio/SndFX/DeadSoundMusic.DeadSoundMusic" 1.0 1.0 0.0 null null))
        (:`then_1`
          (set `self.CanSee` false)
          (set `self.TargetOnOff` true)
          (set `self.GoToNoise` true)
          (`MovementComponent.StopMovementImmediately` (`self.CharacterMovement`))
          (`self.K2_SetActorRotation` (`KismetMathLibrary.MakeRotator` 0.0 0.0 _returnvalue_yaw))
          (`|ExecutionSequence`
            (:`then_0`
              (`KismetSystemLibrary.Delay` 0.2)
              (`|ExecutionSequence`
                (:`then_0`
                  (`SkeletalMeshComponent.PlayAnimation` (`self.Mesh`) (`|GetArrayItem` _killanimarray (`KismetMathLibrary.RandomIntegerInRange` 0 (`KismetArrayLibrary.Array_LastIndex` _killanimarray))) false) ; PlayRandomKillAnim
                  (`KismetSystemLibrary.Delay` 0.5)
                  (bind _returnvalue (`|CreateWidget` "/Game/Widgets/DeadWidget.DeadWidget_C"))
                  (`UserWidget.AddToViewport` _returnvalue 0))
                (:`then_1`
                  (`KismetSystemLibrary.Delay` 0.2)
                  (`PlayerCameraManager.StartCameraFade` :`self` (`GameplayStatics.GetPlayerCameraManager` 0) :`ToAlpha` 1.0 :`Duration` 3.0 :`bHoldWhenFinished` true)
                  (goto _label :!via `Open`))))
            (:`then_1`
              ;;[1 1 1] MakeFallDownQuestObjInHand
              (bind _asquest_obj_1 (cast `/Game/Blueprints/QuestObj/QuestObj1` (`/Game/FirstPersonBP/Blueprints/FirstPersonCharacter.UnderAimActor` (cast `/Game/FirstPersonBP/Blueprints/FirstPersonCharacter` (`GameplayStatics.GetPlayerPawn` 0) :!pure true))))
              (`/Game/Blueprints/QuestObj/QuestObj1.questObjRelease` _asquest_obj_1))))))))

(event `EventTickDeath`
  (params (DeltaSeconds :type "Float (double-precision)"))
  ;[1 0.02604 0.02604] AiWin
  (`|ExecutionSequence`
    (:`then_0`
      (`/Engine/EditorBlueprintResources/StandardMacros.Gate` true :!label _label
        (:`Exit`
          (set `CameraComponent.FieldOfView` (`KismetMathLibrary.Lerp` (`CameraComponent.FieldOfView` (`self.CameraAi`)) 50.0 DeltaSeconds) (`self.CameraAi`)))))))

(event `RunToLastPlayerLoc`
  (bind _player (`self.player`))
  (bind _playerlastloconnavmesh (`/Game/FirstPersonBP/Blueprints/FirstPersonCharacter.PlayerLastLocOnNavMesh` _player))
  ;[0.2118 0.6154 1] ChaseIfPlayerInCloset
  (`/Engine/EditorBlueprintResources/StandardMacros.DoOnce` false :!label _label_2
    (:`Completed`
      (`|ExecutionSequence`
        (:`then_0`
          (`/Game/FirstPersonBP/Blueprints/FirstPersonCharacter.LastLocNavMesh` _player :!label _label_3)
          (set `CharacterMovementComponent.MaxWalkSpeed` (`self.ChaseRunSpeed`) (`self.CharacterMovement`) :!label _label_4) ; 350
          (if (== _playerlastloconnavmesh (0.0 0.0 0.0) :`ErrorTolerance` 0.1)
            (goto _label_3)
            (else
              (`|AIMoveTo` self _playerlastloconnavmesh null
                (:`then`
                  (`/Engine/EditorBlueprintResources/StandardMacros.DoOnce` false :!label _label_5
                    (:`Completed`
                      (`AudioComponent.Play` (`self.MonstrVoice`) 0.0)
                      (bind _asmonster_1animation (cast `/Game/Geometry/char/Enemy1/Monster1Animation` (`SkeletalMeshComponent.GetAnimInstance` (`self.Mesh`))))
                      (set `/Game/Geometry/char/Enemy1/Monster1Animation.HeadRotationFloat` 1.0 _asmonster_1animation)
                      (set `/Game/Geometry/char/Enemy1/Monster1Animation.HeadRotationFloat2` 0.2 _asmonster_1animation)
                      (set `/Game/Geometry/char/Enemy1/Monster1Animation.HeadRotationFloat3` 0.4 _asmonster_1animation)
                      (`/Game/FirstPersonBP/Blueprints/FirstPersonCharacter.MonsterSawU` (`self.player`)) ; Counter
                    )))
                (:`OnSuccess`
                  (set `self.Can hear` true)
                  (set `self.GoToNoise` false)
                  (set `self.TargetOnOff` false)
                  (`KismetSystemLibrary.Delay` 3.0)
                  (`|AIMoveTo` self (0.0 0.0 0.0) (`self.player`) 200.0 ; default 300
                    (:`OnSuccess`
                      (`self.Patrol`)
                      (`|ExecutionSequence`
                        (:`then_0`
                          (goto _label_5 :!via `Reset`))
                        (:`then_1`
                          (goto _label_2 :!via `Reset`))))
                    (:`OnFail`
                      (set `self.Fails` (+ (`self.Fails`) 1) :!label _label_6)
                      (goto _label_4))))
                (:`OnFail`
                  (if (< (`self.Fails`) 3)
                    (goto _label_6)
                    (else
                      (set `self.GoToNoise` false)
                      (set `self.TargetOnOff` false)
                      (`self.Patrol`))))))))
        (:`then_1`
          (`KismetSystemLibrary.RetriggerableDelay` 0.6)
          (goto _label_2 :!via `Reset`))))))

(event `UnderBedKill`
  (bind (_returnvalue_roll _returnvalue_pitch _returnvalue_yaw) (`KismetMathLibrary.BreakRotator` (`KismetMathLibrary.FindLookAtRotation` (`self.K2_GetActorLocation`) (`self.K2_GetActorLocation` (`self.player`)))))
  ;[0.2865 0 0.01168] AiWinUnderBed
  (`/Engine/EditorBlueprintResources/StandardMacros.DoOnce` false
    (:`Completed`
      (`|ExecutionSequence`
        (:`then_0`
          (`GameplayStatics.PlaySound2D` "/Game/Audio/SndFX/DeadSoundMusic.DeadSoundMusic" 1.0 1.0 0.0 null null)
          (`SceneComponent.K2_SetWorldTransform` (`self.CameraAi`) (`SceneComponent.K2_GetComponentToWorld` (`self.Arrow4UnderBed`)) false true))
        (:`then_1`
          (set `self.CanSee` false)
          (set `self.TargetOnOff` true)
          (set `self.GoToNoise` true)
          (`MovementComponent.StopMovementImmediately` (`self.CharacterMovement`))
          (`self.K2_SetActorRotation` (`KismetMathLibrary.MakeRotator` 0.0 0.0 _returnvalue_yaw))
          (`KismetSystemLibrary.Delay` 0.2)
          (`|ExecutionSequence`
            (:`then_0`
              (`SkeletalMeshComponent.PlayAnimation` (`self.Mesh`) "/Game/Geometry/char/Enemy1/Anim/UnderBedDead.UnderBedDead" false)
              (`KismetSystemLibrary.Delay` 1.0)
              (bind _returnvalue (`|CreateWidget` "/Game/Widgets/DeadWidget.DeadWidget_C"))
              (`UserWidget.AddToViewport` _returnvalue 0))
            (:`then_1`
              (`KismetSystemLibrary.Delay` 0.5)
              (`PlayerCameraManager.StartCameraFade` :`self` (`GameplayStatics.GetPlayerCameraManager` 0) :`ToAlpha` 1.0 :`Duration` 3.0 :`bHoldWhenFinished` true)
              (goto _label_7 :!via `Open`))))))))

(event `EventTickUnderBed`
  (params (DeltaSeconds :type "Float (double-precision)"))
  ;[0.2865 0 0.01168] AiWinUnderBed
  (`|ExecutionSequence`
    (:`then_0`
      (`/Engine/EditorBlueprintResources/StandardMacros.Gate` true :!label _label_7
        (:`Exit`
          (set `CameraComponent.FieldOfView` (`KismetMathLibrary.Lerp` (`CameraComponent.FieldOfView` (`self.CameraAi`)) 50.0 DeltaSeconds) (`self.CameraAi`)))))))

(event `StandartChaseEvent`
  ;[0.3438 0.213 0.03485] StandartChase
  (bind _outhit (`KismetSystemLibrary.LineTraceSingle` :`Start` (`self.K2_GetActorLocation`) :`End` (`self.K2_GetActorLocation` (`self.player`)) :`TraceChannel` "TraceTypeQuery1" :`bTraceComplex` true :`DrawTime` 0.0))
  (bind (_bblockinghit _binitialoverlap _time _distance _location _impactpoint _normal _impactnormal _physmat _hitactor _hitcomponent _hitbonename _hititem _faceindex _tracestart _traceend) (`GameplayStatics.BreakHitResult` _outhit))
  (if (not (== _traceend (0.0 0.0 0.0) :`ErrorTolerance` 0.01))
    (set `CharacterMovementComponent.MaxWalkSpeed` (`self.ChaseRunSpeed`) (`self.CharacterMovement`)) ; 350
    (`|AIMoveTo` self _traceend null 10.0
      (:`then`
        (`/Engine/EditorBlueprintResources/StandardMacros.DoOnce` false :!label _label_8
          (:`Completed`
            (`AudioComponent.Play` (`self.MonstrVoice`) 0.0)
            (bind _asmonster_1animation (cast `/Game/Geometry/char/Enemy1/Monster1Animation` (`SkeletalMeshComponent.GetAnimInstance` (`self.Mesh`))))
            (set `/Game/Geometry/char/Enemy1/Monster1Animation.HeadRotationFloat` 1.0 _asmonster_1animation)
            (set `/Game/Geometry/char/Enemy1/Monster1Animation.HeadRotationFloat2` 0.2 _asmonster_1animation)
            (set `/Game/Geometry/char/Enemy1/Monster1Animation.HeadRotationFloat3` 0.4 _asmonster_1animation)
            (`/Game/FirstPersonBP/Blueprints/FirstPersonCharacter.MonsterSawU` (`self.player`)) ; Counter
          )))
      (:`OnSuccess`
        (`|ExecutionSequence`
          (:`then_0`
            (set `self.Can hear` true)
            (set `self.GoToNoise` false)
            (set `self.TargetOnOff` false)
            (`KismetSystemLibrary.Delay` 4.5)
            (`self.Patrol`)
            (goto _label_8 :!via `Reset`)))))))

(event `EventTickDevPrintString`
  ;[0 0 0] Dev Block
  (`/Engine/EditorBlueprintResources/StandardMacros.IsValid` (`self.player`)
    (:`Is Valid`
      (`KismetSystemLibrary.PrintString` (`KismetTextLibrary.Conv_TextToString` (`|FormatText` "Target - {bool}" (`KismetTextLibrary.Conv_BoolToText` (`self.TargetOnOff`)))) true true (struct :`G` 0.66 :`B` 1.0 :`A` 1.0) 0.005)
      (`KismetSystemLibrary.PrintString` (`KismetTextLibrary.Conv_TextToString` (`|FormatText` "Go To Noise - {bool}" (`KismetTextLibrary.Conv_BoolToText` (`self.GoToNoise`)))) true true (struct :`R` 0.182687 :`G` 0.014812 :`B` 1.0 :`A` 1.0) 0.005)
      (`KismetSystemLibrary.PrintString` (`KismetTextLibrary.Conv_TextToString` (`|FormatText` "Can See - {bool}" (`KismetTextLibrary.Conv_BoolToText` (`self.CanSee`)))) true true (struct :`R` 0.912919 :`B` 1.0 :`A` 1.0) 0.005)
      (`KismetSystemLibrary.PrintString` (`KismetTextLibrary.Conv_TextToString` (`|FormatText` "Go To Noise Obj - {bool}" (`KismetTextLibrary.Conv_BoolToText` (`self.GoToNoiseObj`)))) true true (struct :`G` 1.0 :`B` 0.499694 :`A` 1.0) 0.005)
      (`KismetSystemLibrary.PrintString` (`KismetTextLibrary.Conv_TextToString` (`|FormatText` "Can Hear - {bool}" (`KismetTextLibrary.Conv_BoolToText` (`self.Can hear`)))) true true (struct :`R` 0.390895 :`G` 1.0 :`A` 1.0) 0.005)
      (`KismetSystemLibrary.PrintString` (`KismetTextLibrary.Conv_TextToString` (`|FormatText` "PlayerHidden4Sense - {bool}" (`KismetTextLibrary.Conv_BoolToText` (`/Game/FirstPersonBP/Blueprints/FirstPersonCharacter.PlayerHiddenForSense` (`self.player`))))) true true (struct :`R` 0.991265 :`G` 1.0 :`A` 1.0) 0.005)
      (`KismetSystemLibrary.PrintString` (`KismetSystemLibrary.GetDisplayName` (`self.player`)) true true (struct :`R` 1.0 :`G` 0.531514 :`A` 1.0) 0.005))))

(fn `SaySmthg`
  (`GameplayStatics.PlaySoundAtLocation` "/Game/Audio/SndFX/Monster_Patrol_Phrases_Cue.Monster_Patrol_Phrases_Cue" (`SceneComponent.K2_GetComponentLocation` (`self.Mesh`)) (struct) 1.0 1.0 0.0 "/Game/Audio/SND_Attenuation2.SND_Attenuation2" null null))

(fn `UserConstructionScript`)