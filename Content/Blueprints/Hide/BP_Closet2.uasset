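; BP_Closet2 is a hiding closet with a sliding door that the enemy can flush the player out of.
; OpenCloseDoor toggles the door through a FlipFlop, sharing its opening move and sound with DoorOpenOnly.
; An inner box overlap flags the player as hidden for the chase system.
; When AiEnemy1 enters Box4Enemy with the player inside, the door opens and, after short delays, the player teleports to the Arrow.
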(event `DoorOpenOnly`
  ;[0.3542 0.1417 0.08124] OpenCloseEvent
  (if (`self.isDoorClosed?`)
    (`GameplayStatics.PlaySoundAtLocation` "/Game/Audio/SndFX/OpenDoor1_Cue.OpenDoor1_Cue" (`SceneComponent.K2_GetComponentLocation` (`self.Closet2_Door`)) (struct) 1.0 1.0 0.0 "/Game/Audio/SND_Attenuation1.SND_Attenuation1" null null :!label _label)
    (`KismetSystemLibrary.MoveComponentTo` (`self.Closet2_Door`) (0.0 36.0 125.900002) (struct) true true 0.65)
    (set `self.isDoorClosed?` false)))

(event `OpenCloseDoor`
  ;[0.3542 0.1417 0.08124] OpenCloseEvent
  (`/Engine/EditorBlueprintResources/StandardMacros.FlipFlop`
    (:`A`
      (goto _label))
    (:`B`
      (`GameplayStatics.PlaySoundAtLocation` "/Game/Audio/SndFX/OpenDoor1_Cue.OpenDoor1_Cue" (`SceneComponent.K2_GetComponentLocation` (`self.Closet2_Door`)) (struct) 1.0 1.0 0.0 "/Game/Audio/SND_Attenuation1.SND_Attenuation1" null null)
      (`KismetSystemLibrary.MoveComponentTo` (`self.Closet2_Door`) (-62.0 36.0 125.900002) (struct) true true 0.65)
      (set `self.isDoorClosed?` true))))

(event `self.Box.OnComponentBeginOverlap`
  (params (OverlappedComponent :type "PrimitiveComponent Object Reference") (OtherActor :type "Actor Object Reference") (OtherComp :type "PrimitiveComponent Object Reference") (OtherBodyIndex :type Integer) (bFromSweep :type Boolean) (SweepResult :type "HitResult Structure (by ref)"))
  ;[0.0769 0.2443 1] HideShowEvents
  (bind _asfirst_person_character (cast `/Game/FirstPersonBP/Blueprints/FirstPersonCharacter` OtherActor))
  (set `self.PlayerAtCloset` _asfirst_person_character)
  (set `self.PlayerInCloset` true)
  (set `/Game/FirstPersonBP/Blueprints/FirstPersonCharacter.IsPlayerHiddenCloset` true (`self.PlayerAtCloset`)) ; NeedForChooseChaseSystem
)

(event `self.Box.OnComponentEndOverlap`
  (params (OverlappedComponent :type "PrimitiveComponent Object Reference") (OtherActor :type "Actor Object Reference") (OtherComp :type "PrimitiveComponent Object Reference") (OtherBodyIndex :type Integer))
  ;[0.0769 0.2443 1] HideShowEvents
  (cast `/Game/FirstPersonBP/Blueprints/FirstPersonCharacter` OtherActor)
  (set `self.PlayerInCloset` false)
  (set `/Game/FirstPersonBP/Blueprints/FirstPersonCharacter.IsPlayerHiddenCloset` false (`self.PlayerAtCloset`))
  (set `self.PlayerAtCloset` (`self.PlayerNull`)))

(event `self.Box4Enemy.OnComponentBeginOverlap`
  (params (OverlappedComponent :type "PrimitiveComponent Object Reference") (OtherActor :type "Actor Object Reference") (OtherComp :type "PrimitiveComponent Object Reference") (OtherBodyIndex :type Integer) (bFromSweep :type Boolean) (SweepResult :type "HitResult Structure (by ref)"))
  (bind (_returnvalue_location _returnvalue_rotation) (`KismetMathLibrary.BreakTransform` (`SceneComponent.K2_GetComponentToWorld` (`self.Arrow`))))
  ;[0.4271 0.06107 0.04407] TeleportPlayerCloserToEnemy
  (cast `/Game/Blueprints/AI1BP/AiEnemy1` OtherActor)
  (if (`self.PlayerInCloset`)
    (`|ExecutionSequence`
      (:`then_0`
        ;;[1 1 1] ToOpenDoor
        (if (`self.isDoorClosed?`)
          (`self.DoorOpenOnly`)))
      (:`then_1`
        (`KismetSystemLibrary.Delay` 0.7)
        (for _ (range 11)
          (`KismetSystemLibrary.Delay` 0.5)
          (`self.K2_TeleportTo` (`self.PlayerAtCloset`) _returnvalue_location _returnvalue_rotation))))))

(fn `UserConstructionScript`)