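; BP_Bed is a hiding spot that the player can crawl under to evade AiEnemy1.
; A flip-flop event shrinks the player to an arrow marker with collision and touch controls changed, then restores the saved transform on exit.
; The player counts as hidden only if the enemy had no target on entry; otherwise an enemy overlapping the box triggers a delayed under-bed kill.
; The construction script applies a custom mesh and box sizing.
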(event `SetPlayer`
  ;[0.05872 0.1026 0.4271] SetPlayer
  (if (`self.Bed_On/off`)
    (bind _asfirst_person_character (cast `/Game/FirstPersonBP/Blueprints/FirstPersonCharacter` (`GameplayStatics.GetPlayerPawn` 0)))
    (set `self.PlayerAtBed` _asfirst_person_character)))

(event `HideUnhideUnderBedEvent`
  (bind _playeratbed (`self.PlayerAtBed`))
  (bind _playeratbed_2 (`self.PlayerAtBed`))
  (bind _arrow (`self.Arrow`))
  (bind _playeratbed_3 (`self.PlayerAtBed`))
  (bind (_returnvalue_location _returnvalue_rotation) (`KismetMathLibrary.BreakTransform` (`SceneComponent.K2_GetComponentToWorld` _arrow)))
  ;[0.02506 0.2031 0.1433] HideUnhideUnderBedEvent
  (if (`self.Bed_On/off`)
    (`/Engine/EditorBlueprintResources/StandardMacros.FlipFlop`
      (:`A`
        (set `/Game/FirstPersonBP/Blueprints/FirstPersonCharacter.IsPlayerUnderBed?` true _playeratbed_3)
        (`self.SetActorEnableCollision` _playeratbed_3 false)
        (`PlayerController.ActivateTouchInterface` (`GameplayStatics.GetPlayerController` 0) null)
        (set `self.PlayerLastTransform` (`SceneComponent.K2_GetComponentToWorld` (`Character.CapsuleComponent` _playeratbed_3)))
        (`self.K2_SetActorTransform` _playeratbed_3 (`KismetMathLibrary.MakeTransform` _returnvalue_location _returnvalue_rotation (0.15 0.15 0.15)) false false)
        (`self.K2_SetActorRotation` _playeratbed_3 (`SceneComponent.K2_GetComponentRotation` _arrow) false)
        (set `self.PlayerUnderBed` true)
        (`/Game/Widgets/MainWidget.showDoorOpenButton` (`/Game/FirstPersonBP/Blueprints/FirstPersonCharacter.MainWidget` _playeratbed_3))
        (if (not (`/Game/Blueprints/AI1BP/AiEnemy1.TargetOnOff` (`/Game/FirstPersonBP/Blueprints/FirstPersonCharacter.AiEnemy1` _playeratbed)))
          (set `/Game/FirstPersonBP/Blueprints/FirstPersonCharacter.PlayerHiddenForSense` true _playeratbed)))
      (:`B`
        (`self.K2_SetActorTransform` _playeratbed_2 (`self.PlayerLastTransform`) false false)
        (set `self.PlayerUnderBed` false)
        (set `/Game/FirstPersonBP/Blueprints/FirstPersonCharacter.IsPlayerUnderBed?` false _playeratbed_2)
        (`self.SetActorEnableCollision` _playeratbed_2 true)
        (`PlayerController.ActivateTouchInterface` (`GameplayStatics.GetPlayerController` 0) "/Engine/MobileResources/HUD/LeftVirtualJoystickOnly.LeftVirtualJoystickOnly")
        (set `/Game/FirstPersonBP/Blueprints/FirstPersonCharacter.PlayerHiddenForSense` false (`self.PlayerAtBed`))))))

(event `self.Box.OnComponentBeginOverlap`
  (params (OverlappedComponent :type "PrimitiveComponent Object Reference") (OtherActor :type "Actor Object Reference") (OtherComp :type "PrimitiveComponent Object Reference") (OtherBodyIndex :type Integer) (bFromSweep :type Boolean) (SweepResult :type "HitResult Structure (by ref)"))
  ;[0.3646 0 0.002976] DeathEvent
  (bind _asai_enemy_1 (cast `/Game/Blueprints/AI1BP/AiEnemy1` OtherActor))
  (`KismetSystemLibrary.RetriggerableDelay` 3.0)
  (if (and (`self.PlayerUnderBed`) (not (`/Game/FirstPersonBP/Blueprints/FirstPersonCharacter.PlayerHiddenForSense` (`self.PlayerAtBed`))))
    (`/Game/FirstPersonBP/Blueprints/FirstPersonCharacter.UnderBedDeathEvent` (`self.PlayerAtBed`))
    (`/Game/Blueprints/AI1BP/AiEnemy1.UnderBedKill` _asai_enemy_1)))

(fn `UserConstructionScript`
  (`StaticMeshComponent.SetStaticMesh` (`self.bedMesh`) (`self.BedMeshCustom`))
  (`SceneComponent.SetRelativeScale3D` (`self.Box`) (`self.CollBoxScale`))
  (`SceneComponent.K2_AddLocalOffset` (`self.Box`) (`self.CollBoxOffset`) false false))