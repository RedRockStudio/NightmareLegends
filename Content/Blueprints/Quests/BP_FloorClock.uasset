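; Quest puzzle floor clock with a swinging timeline-driven pendulum and hour and minute hands that start hidden.
; Box overlap shows progress-based tips to an empty-handed player.
; When a tagged QuestObj1 hand overlaps, it destroys the player's aimed-at quest object, reveals that hand and increments Arrows.
; Tick polls the count and, once both are placed, plays a sound and moves the clock door open a single time.
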(event `self.ReceiveTick`
  (params (DeltaSeconds :type "Float (single-precision)"))
  (if (>= (`self.Arrows`) 2)
    (`/Engine/EditorBlueprintResources/StandardMacros.DoOnce` false
      (:`Completed`
        (`GameplayStatics.PlaySoundAtLocation` "/Game/Audio/SndFX/bookFlip2.bookFlip2" (`SceneComponent.K2_GetComponentLocation` (`self.FC_HArrow`)) (struct) 1.0 1.0 0.0 "/Game/Audio/SND_Attenuation1.SND_Attenuation1" null null)
        (`KismetSystemLibrary.MoveComponentTo` (`self.FloorClock_Door`) (0.0 10.0 0.2) (struct :`Roll` -90.0) true true 1.0)))))

(event `self.ReceiveBeginPlay`
  (bind (_direction _pendumul) (`Timeline|TL_Pendumlum` :!via `PlayFromStart`)
    (:`Update`
      (`KismetSystemLibrary.MoveComponentTo` (`self.FloolClockPend`) (0.0 0.0 152.0) (`KismetMathLibrary.MakeRotator` 0.0 (`KismetMathLibrary.Lerp` -12.0 12.0 _pendumul)) true true 0.1 true))))

(event `self.Box.OnComponentBeginOverlap`
  (params (OverlappedComponent :type "PrimitiveComponent Object Reference") (OtherActor :type "Actor Object Reference") (OtherComp :type "PrimitiveComponent Object Reference") (OtherBodyIndex :type Integer) (bFromSweep :type Boolean) (SweepResult :type "HitResult Structure (by ref)"))
  (bind _fc_harrow (`self.FC_HArrow`))
  (`|ExecutionSequence`
    (:`then_0`
      ;[0.2102 0.3762 0.651] Tips
      (bind _asfirst_person_character (cast `/Game/FirstPersonBP/Blueprints/FirstPersonCharacter` OtherActor))
      (if (and (`/Game/FirstPersonBP/Blueprints/FirstPersonCharacter.IsHandEmpty?` _asfirst_person_character) (< (`self.Arrows`) 2))
        (if (== (`self.Arrows`) 1)
          (bind _mainwidget (`/Game/FirstPersonBP/Blueprints/FirstPersonCharacter.MainWidget` _asfirst_person_character))
          (set `/Game/Widgets/MainWidget.CurrTipName` "Clock2" _mainwidget)
          (`/Game/Widgets/MainWidget.Tips` _mainwidget)
          (else
            (set `/Game/Widgets/MainWidget.CurrTipName` "Clock1" _mainwidget)
            (`/Game/Widgets/MainWidget.Tips` _mainwidget)))))
    (:`then_1`
      (bind _asquest_obj_1 (cast `/Game/Blueprints/QuestObj/QuestObj1` OtherActor))
      (`|ExecutionSequence`
        (:`then_0`
          (if (`self.ActorHasTag` _asquest_obj_1 "QO_ClockHour")
            (bind _asquest_obj_1_2 (cast `/Game/Blueprints/QuestObj/QuestObj1` (`/Game/FirstPersonBP/Blueprints/FirstPersonCharacter.UnderAimActor` (cast `/Game/FirstPersonBP/Blueprints/FirstPersonCharacter` (`GameplayStatics.GetPlayerPawn` 0) :!pure true))))
            (`self.K2_DestroyActor` _asquest_obj_1_2)
            (`SceneComponent.SetVisibility` _fc_harrow true false)
            (`|ExecutionSequence`
              (:`then_0`
                (set `self.Arrows` (+ (`self.Arrows`) 1)))
              (:`then_1`
                (`GameplayStatics.PlaySoundAtLocation` "/Game/Audio/SndFX/takeMetObj.takeMetObj" (`SceneComponent.K2_GetComponentLocation` _fc_harrow) (struct) 1.0 1.0 0.0 "/Game/Audio/SND_Attenuation1.SND_Attenuation1" null null :!label _label)))))
        (:`then_1`
          (if (`self.ActorHasTag` _asquest_obj_1 "QO_ClockMin")
            (bind _asquest_obj_1_3 (cast `/Game/Blueprints/QuestObj/QuestObj1` (`/Game/FirstPersonBP/Blueprints/FirstPersonCharacter.UnderAimActor` (cast `/Game/FirstPersonBP/Blueprints/FirstPersonCharacter` (`GameplayStatics.GetPlayerPawn` 0) :!pure true))))
            (`self.K2_DestroyActor` _asquest_obj_1_3)
            (`SceneComponent.SetVisibility` (`self.FC_MArrow`) true false)
            (`|ExecutionSequence`
              (:`then_0`
                (goto _label))
              (:`then_1`
                (set `self.Arrows` (+ (`self.Arrows`) 1))))))))))

(fn `UserConstructionScript`
  (`SceneComponent.SetVisibility` (`self.FC_MArrow`) false false)
  (`SceneComponent.SetVisibility` (`self.FC_HArrow`) false false))