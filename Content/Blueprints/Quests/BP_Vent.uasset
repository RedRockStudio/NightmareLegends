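; Two-stage vent quest actor where a screwdriver removes the cage, then wirecutters cut the wire.
; Box overlap shows state-based tips to an empty-handed player and detects tagged QuestObj1 tools, destroying the player's aimed-at object and revealing a built-in tool mesh.
; Chained timelines, MoveComponentTo and delays spin out four bolts before the cage falls with physics.
; Wirecutters, gated by CageRemoved, play three animated cuts, swap in the cut-wire mesh and set QuestDone.
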(event `self.Box.OnComponentBeginOverlap`
  (params (OverlappedComponent :type "PrimitiveComponent Object Reference") (OtherActor :type "Actor Object Reference") (OtherComp :type "PrimitiveComponent Object Reference") (OtherBodyIndex :type Integer) (bFromSweep :type Boolean) (SweepResult :type "HitResult Structure (by ref)"))
  (bind _bolt1 (`self.Bolt1`))
  (bind _bolt4 (`self.Bolt4`))
  (bind _ventcage (`self.VentCage`))
  (bind _bolt3 (`self.Bolt3`))
  (bind _bolt2 (`self.Bolt2`))
  (bind _wirecutter (`self.wireCutter`))
  (bind _wirecutted (`self.wireCutted`))
  (bind _screwdriver (`self.Screwdriver`))
  (bind _wirecutter_2 (`self.wireCutter`))
  (`|ExecutionSequence`
    (:`then_0`
      ;[0.2102 0.3762 0.651] Tips
      (bind _asfirst_person_character (cast `/Game/FirstPersonBP/Blueprints/FirstPersonCharacter` OtherActor))
      (if (and (`/Game/FirstPersonBP/Blueprints/FirstPersonCharacter.IsHandEmpty?` _asfirst_person_character) (not (`self.QuestDone`)))
        (if (`self.CageRemoved`)
          (bind _mainwidget (`/Game/FirstPersonBP/Blueprints/FirstPersonCharacter.MainWidget` _asfirst_person_character))
          (set `/Game/Widgets/MainWidget.CurrTipName` "Vent2" _mainwidget)
          (`/Game/Widgets/MainWidget.Tips` _mainwidget)
          (else
            (set `/Game/Widgets/MainWidget.CurrTipName` "Vent1" _mainwidget)
            (`/Game/Widgets/MainWidget.Tips` _mainwidget)))))
    (:`then_1`
      (bind _asquest_obj_1 (cast `/Game/Blueprints/QuestObj/QuestObj1` OtherActor))
      (`|ExecutionSequence`
        (:`then_0`
          (if (`self.ActorHasTag` _asquest_obj_1 "QO_Screwdriver")
            (set `self.CageRemoved` true)
            (bind _asquest_obj_1_2 (cast `/Game/Blueprints/QuestObj/QuestObj1` (`/Game/FirstPersonBP/Blueprints/FirstPersonCharacter.UnderAimActor` (cast `/Game/FirstPersonBP/Blueprints/FirstPersonCharacter` (`GameplayStatics.GetPlayerPawn` 0) :!pure true))))
            (`self.K2_DestroyActor` _asquest_obj_1_2)
            (`SceneComponent.SetVisibility` _screwdriver true false)
            (`GameplayStatics.PlaySoundAtLocation` "/Game/Audio/SndFX/Screwdriver_Spin.Screwdriver_Spin" (`SceneComponent.K2_GetComponentLocation` (`self.VentCage`)) (struct) 1.0 1.0 0.0 "/Game/Audio/SND_Attenuation1.SND_Attenuation1" null null)
            (bind (_direction _rotate) (`Timeline|rotateScrew` :!via `PlayFromStart`)
              (:`Update`
                (`SceneComponent.K2_AddRelativeRotation` (`self.Screwdriver`) (`KismetMathLibrary.MakeRotator` _rotate) false false)
                (`SceneComponent.K2_AddRelativeRotation` (`self.Bolt1`) (`KismetMathLibrary.MakeRotator` _rotate) false false))
              (:`Finished`
                (`|ExecutionSequence`
                  (:`then_0`
                    (`KismetSystemLibrary.Delay` 0.5)
                    (`KismetSystemLibrary.MoveComponentTo` _screwdriver (22.154263 19.895123 20.84903) (struct :`Yaw` -90.0) true true 0.5)
                    (`KismetSystemLibrary.Delay` 0.3)
                    (`GameplayStatics.PlaySoundAtLocation` "/Game/Audio/SndFX/Screwdriver_Spin.Screwdriver_Spin" (`SceneComponent.K2_GetComponentLocation` (`self.VentCage`)) (struct) 1.0 1.0 0.0 "/Game/Audio/SND_Attenuation1.SND_Attenuation1" null null)
                    (bind (_direction_2 _rotate_2) (`Timeline|Timeline_0` :!via `PlayFromStart`)
                      (:`Update`
                        (`SceneComponent.K2_AddRelativeRotation` (`self.Screwdriver`) (`KismetMathLibrary.MakeRotator` _rotate_2) false false)
                        (`SceneComponent.K2_AddRelativeRotation` (`self.Bolt4`) (`KismetMathLibrary.MakeRotator` _rotate_2) false false))
                      (:`Finished`
                        (`|ExecutionSequence`
                          (:`then_0`
                            (`KismetSystemLibrary.Delay` 0.5)
                            (`KismetSystemLibrary.MoveComponentTo` (`self.Screwdriver`) (-22.0 20.0 20.700001) (struct :`Yaw` -90.0) true true 0.5)
                            (`KismetSystemLibrary.Delay` 0.3)
                            (`GameplayStatics.PlaySoundAtLocation` "/Game/Audio/SndFX/Screwdriver_Spin.Screwdriver_Spin" (`SceneComponent.K2_GetComponentLocation` (`self.VentCage`)) (struct) 1.0 1.0 0.0 "/Game/Audio/SND_Attenuation1.SND_Attenuation1" null null)
                            (bind (_direction_3 _rotate_3) (`Timeline|Timeline_1` :!via `PlayFromStart`)
                              (:`Update`
                                (`SceneComponent.K2_AddRelativeRotation` (`self.Screwdriver`) (`KismetMathLibrary.MakeRotator` _rotate_3) false false)
                                (`SceneComponent.K2_AddRelativeRotation` (`self.Bolt3`) (`KismetMathLibrary.MakeRotator` _rotate_3) false false))
                              (:`Finished`
                                (`|ExecutionSequence`
                                  (:`then_0`
                                    (`KismetSystemLibrary.Delay` 0.5)
                                    (`KismetSystemLibrary.MoveComponentTo` (`self.Screwdriver`) (-22.0 20.0 -21.0) (struct :`Yaw` -90.0) true true 0.5)
                                    (`KismetSystemLibrary.Delay` 0.3)
                                    (`GameplayStatics.PlaySoundAtLocation` "/Game/Audio/SndFX/Screwdriver_Spin.Screwdriver_Spin" (`SceneComponent.K2_GetComponentLocation` (`self.VentCage`)) (struct) 1.0 1.0 0.0 "/Game/Audio/SND_Attenuation1.SND_Attenuation1" null null)
                                    (bind (_direction_4 _rotate_4) (`Timeline|Timeline_2` :!via `PlayFromStart`)
                                      (:`Update`
                                        (`SceneComponent.K2_AddRelativeRotation` (`self.Screwdriver`) (`KismetMathLibrary.MakeRotator` _rotate_4) false false)
                                        (`SceneComponent.K2_AddRelativeRotation` (`self.Bolt2`) (`KismetMathLibrary.MakeRotator` _rotate_4) false false))
                                      (:`Finished`
                                        (`|ExecutionSequence`
                                          (:`then_0`
                                            (`PrimitiveComponent.SetSimulatePhysics` _bolt2 true)
                                            (`PrimitiveComponent.SetCollisionEnabled` _bolt2 "PhysicsOnly")
                                            (`KismetSystemLibrary.Delay` 3.0)
                                            (`ActorComponent.K2_DestroyComponent` _bolt2))
                                          (:`then_1`
                                            (`GameplayStatics.PlaySoundAtLocation` "/Game/Audio/SndFX/metal_int1.metal_int1" (`SceneComponent.K2_GetComponentLocation` (`self.VentCage`)) (struct) 1.0 1.0 0.0 "/Game/Audio/SND_Attenuation1.SND_Attenuation1" null null)
                                            (`PrimitiveComponent.SetSimulatePhysics` _ventcage true)
                                            (`PrimitiveComponent.SetCollisionEnabled` _ventcage "PhysicsOnly")
                                            (`KismetSystemLibrary.Delay` 0.4)
                                            (`GameplayStatics.PlaySoundAtLocation` "/Game/Audio/SndFX/metal_int2.metal_int2" (`SceneComponent.K2_GetComponentLocation` _ventcage) (struct) 1.0 1.0 0.0 "/Game/Audio/SND_Attenuation1.SND_Attenuation1" null null)
                                            (`KismetSystemLibrary.Delay` 4.0)
                                            (`PrimitiveComponent.SetSimulatePhysics` _ventcage false))
                                          (:`then_2`
                                            (`ActorComponent.K2_DestroyComponent` (`self.Screwdriver`)))))))
                                  (:`then_1`
                                    (`PrimitiveComponent.SetSimulatePhysics` _bolt3 true)
                                    (`PrimitiveComponent.SetCollisionEnabled` _bolt3 "PhysicsOnly")
                                    (`KismetSystemLibrary.Delay` 3.0)
                                    (`ActorComponent.K2_DestroyComponent` _bolt3))))))
                          (:`then_1`
                            (`PrimitiveComponent.SetSimulatePhysics` _bolt4 true)
                            (`PrimitiveComponent.SetCollisionEnabled` _bolt4 "PhysicsOnly")
                            (`KismetSystemLibrary.Delay` 3.0)
                            (`ActorComponent.K2_DestroyComponent` _bolt4))))))
                  (:`then_1`
                    (`PrimitiveComponent.SetSimulatePhysics` _bolt1 true)
                    (`PrimitiveComponent.SetCollisionEnabled` _bolt1 "PhysicsOnly")
                    (`KismetSystemLibrary.Delay` 3.0)
                    (`ActorComponent.K2_DestroyComponent` _bolt1)))))))
        (:`then_1`
          (if (and (`self.ActorHasTag` _asquest_obj_1 "QO_Wirecutter") (`self.CageRemoved`))
            (set `self.QuestDone` true)
            (bind _asquest_obj_1_3 (cast `/Game/Blueprints/QuestObj/QuestObj1` (`/Game/FirstPersonBP/Blueprints/FirstPersonCharacter.UnderAimActor` (cast `/Game/FirstPersonBP/Blueprints/FirstPersonCharacter` (`GameplayStatics.GetPlayerPawn` 0) :!pure true))))
            (`self.K2_DestroyActor` _asquest_obj_1_3)
            (`SceneComponent.SetVisibility` _wirecutter_2 true false)
            (`KismetSystemLibrary.Delay` 0.2)
            (`|ExecutionSequence`
              (:`then_0`
                (`SkeletalMeshComponent.PlayAnimation` _wirecutter_2 "/Game/Geometry/Props/Anims/wirecutter/wirecutter_Anim.wirecutter_Anim" false)
                (`KismetSystemLibrary.Delay` 1.0)
                (`KismetSystemLibrary.MoveComponentTo` _wirecutter_2 (3.468839 2.615326 7.831015) (struct :`Pitch` 11.5 :`Yaw` -116.400002 :`Roll` 79.599998) true true 0.5)
                (`KismetSystemLibrary.Delay` 0.5)
                (`|ExecutionSequence`
                  (:`then_0`
                    (`SkeletalMeshComponent.PlayAnimation` (`self.wireCutter`) "/Game/Geometry/Props/Anims/wirecutter/wirecutter_Anim.wirecutter_Anim" false)
                    (`KismetSystemLibrary.Delay` 1.0)
                    (`KismetSystemLibrary.MoveComponentTo` (`self.wireCutter`) (-12.263615 3.073822 -5.91109) (struct :`Pitch` 11.5 :`Yaw` -116.400002 :`Roll` 79.599998) true true 0.5)
                    (`KismetSystemLibrary.Delay` 0.2)
                    (`|ExecutionSequence`
                      (:`then_0`
                        (`SkeletalMeshComponent.PlayAnimation` _wirecutter "/Game/Geometry/Props/Anims/wirecutter/wirecutter_Anim.wirecutter_Anim" false)
                        (`KismetSystemLibrary.Delay` 1.0)
                        (`|ExecutionSequence`
                          (:`then_0`
                            (`KismetSystemLibrary.Delay` 0.5)
                            (`ActorComponent.K2_DestroyComponent` _wirecutter))
                          (:`then_1`
                            (`ActorComponent.K2_DestroyComponent` (`self.wire`))
                            (`SceneComponent.SetVisibility` _wirecutted true false)
                            (`GameplayStatics.PlaySoundAtLocation` "/Game/Audio/SndFX/metal_int1.metal_int1" (`SceneComponent.K2_GetComponentLocation` _wirecutted) (struct) 1.0 1.0 0.0 "/Game/Audio/SND_Attenuation1.SND_Attenuation1" null null))))
                      (:`then_1`
                        (`GameplayStatics.PlaySoundAtLocation` "/Game/Audio/SndFX/wireCutter_Cut.wireCutter_Cut" (`SceneComponent.K2_GetComponentLocation` (`self.wireCutter`)) (struct) 1.0 1.0 0.0 "/Game/Audio/SND_Attenuation1.SND_Attenuation1" null null))))
                  (:`then_1`
                    (`GameplayStatics.PlaySoundAtLocation` "/Game/Audio/SndFX/wireCutter_Cut.wireCutter_Cut" (`SceneComponent.K2_GetComponentLocation` (`self.wireCutter`)) (struct) 1.0 1.0 0.0 "/Game/Audio/SND_Attenuation1.SND_Attenuation1" null null))))
              (:`then_1`
                (`GameplayStatics.PlaySoundAtLocation` "/Game/Audio/SndFX/wireCutter_Cut.wireCutter_Cut" (`SceneComponent.K2_GetComponentLocation` (`self.wireCutter`)) (struct) 1.0 1.0 0.0 "/Game/Audio/SND_Attenuation1.SND_Attenuation1" null null)))))))))

(fn `UserConstructionScript`
  (`SceneComponent.SetVisibility` (`self.wireCutted`) false false)
  (`SceneComponent.SetVisibility` (`self.Screwdriver`) false false)
  (`SceneComponent.SetVisibility` (`self.wireCutter`) false false))