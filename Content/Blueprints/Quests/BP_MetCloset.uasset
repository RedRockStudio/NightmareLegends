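; Metal closet quest actor that the player opens in two stages, using green wirecutters and then a key.
; Box overlap shows stage-dependent tips to empty-handed players and checks QuestObj1 tags, accepting the key only after chains are removed.
; Each stage destroys the QuestObj1 under the player's aim and reveals a hidden stand-in component.
; Delay-timed animations, component moves and sounds play the chain cutting and door opening.
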(event `self.Box.OnComponentBeginOverlap`
  (params (OverlappedComponent :type "PrimitiveComponent Object Reference") (OtherActor :type "Actor Object Reference") (OtherComp :type "PrimitiveComponent Object Reference") (OtherBodyIndex :type Integer) (bFromSweep :type Boolean) (SweepResult :type "HitResult Structure (by ref)"))
  (bind _closetchains (`self.closetChains`))
  (bind _wirecutter (`self.wirecutter`))
  (bind _closetkey (`self.ClosetKey`))
  (bind _closet_door (`self.Closet_Door`))
  (bind _returnvalue (`SceneComponent.K2_GetComponentLocation` _closet_door))
  (`|ExecutionSequence`
    (:`then_0`
      ;[0.2102 0.3762 0.651] Tips
      (bind _asfirst_person_character (cast `/Game/FirstPersonBP/Blueprints/FirstPersonCharacter` OtherActor))
      (if (and (`/Game/FirstPersonBP/Blueprints/FirstPersonCharacter.IsHandEmpty?` _asfirst_person_character) (not (`self.QuestDone`)))
        (if (`self.ChainsRemoved`)
          (bind _mainwidget (`/Game/FirstPersonBP/Blueprints/FirstPersonCharacter.MainWidget` _asfirst_person_character))
          (set `/Game/Widgets/MainWidget.CurrTipName` "GreenCloset2" _mainwidget)
          (`/Game/Widgets/MainWidget.Tips` _mainwidget)
          (else
            (set `/Game/Widgets/MainWidget.CurrTipName` "GreenCloset1" _mainwidget)
            (`/Game/Widgets/MainWidget.Tips` _mainwidget)))))
    (:`then_1`
      (bind _asquest_obj_1 (cast `/Game/Blueprints/QuestObj/QuestObj1` OtherActor))
      (`|ExecutionSequence`
        (:`then_0`
          (if (`self.ActorHasTag` _asquest_obj_1 "QO_WirecutterGreen")
            (set `self.ChainsRemoved` true)
            (bind _asquest_obj_1_2 (cast `/Game/Blueprints/QuestObj/QuestObj1` (`/Game/FirstPersonBP/Blueprints/FirstPersonCharacter.UnderAimActor` (cast `/Game/FirstPersonBP/Blueprints/FirstPersonCharacter` (`GameplayStatics.GetPlayerPawn` 0) :!pure true))))
            (`self.K2_DestroyActor` _asquest_obj_1_2)
            (`SceneComponent.SetVisibility` _wirecutter true false)
            (`KismetSystemLibrary.Delay` 0.5)
            (`|ExecutionSequence`
              (:`then_0`
                (`SkeletalMeshComponent.PlayAnimation` _wirecutter "/Game/Geometry/Props/Anims/wirecutter/wirecutter_Anim.wirecutter_Anim" false)
                (`KismetSystemLibrary.Delay` 0.7)
                (`|ExecutionSequence`
                  (:`then_0`
                    (`SkeletalMeshComponent.PlayAnimation` _closetchains "/Game/Geometry/Props/Anims/chains/closetChains_Anim.closetChains_Anim" false)
                    (`KismetSystemLibrary.Delay` 0.5)
                    (`ActorComponent.K2_DestroyComponent` _wirecutter))
                  (:`then_1`
                    (`GameplayStatics.PlaySoundAtLocation` "/Game/Audio/SndFX/ChainsFall.ChainsFall" (`SceneComponent.K2_GetComponentLocation` _closetchains) (struct) 1.0 1.0 0.0 "/Game/Audio/SND_Attenuation1.SND_Attenuation1" null null))))
              (:`then_1`
                (`GameplayStatics.PlaySoundAtLocation` "/Game/Audio/SndFX/wireCutter_Cut.wireCutter_Cut" (`SceneComponent.K2_GetComponentLocation` (`self.wirecutter`)) (struct) 1.0 1.0 0.0 "/Game/Audio/SND_Attenuation1.SND_Attenuation1" null null)))))
        (:`then_1`
          (if (and (`self.ActorHasTag` _asquest_obj_1 "QO_ClosetKey") (`self.ChainsRemoved`))
            (set `self.QuestDone` true)
            (bind _asquest_obj_1_3 (cast `/Game/Blueprints/QuestObj/QuestObj1` (`/Game/FirstPersonBP/Blueprints/FirstPersonCharacter.UnderAimActor` (cast `/Game/FirstPersonBP/Blueprints/FirstPersonCharacter` (`GameplayStatics.GetPlayerPawn` 0) :!pure true))))
            (`self.K2_DestroyActor` _asquest_obj_1_3)
            (`|ExecutionSequence`
              (:`then_0`
                (`SceneComponent.SetVisibility` _closetkey true false)
                (`KismetSystemLibrary.Delay` 1.0)
                (`|ExecutionSequence`
                  (:`then_0`
                    (`KismetSystemLibrary.MoveComponentTo` _closetkey (53.104794 13.151144 1.726913) (struct :`Pitch` 90.0 :`Yaw` 26.559999 :`Roll` 116.559998) true true 0.5 true)
                    (`KismetSystemLibrary.Delay` 1.0)
                    (`|ExecutionSequence`
                      (:`then_0`
                        (`KismetSystemLibrary.MoveComponentTo` _closet_door (-31.700682 22.522598 97.713829) (struct :`Yaw` 94.199997) true true 1.0))
                      (:`then_1`
                        (`GameplayStatics.PlaySoundAtLocation` "/Game/Audio/SndFX/doorClose_3.doorClose_3" _returnvalue (struct) 0.6 1.0 0.0 "/Game/Audio/SND_Attenuation1.SND_Attenuation1" null null))
                      (:`then_2`
                        (`KismetSystemLibrary.Delay` 0.7)
                        (`GameplayStatics.PlaySoundAtLocation` "/Game/Audio/SndFX/metal_int1.metal_int1" _returnvalue (struct) 1.4 1.0 0.0 "/Game/Audio/SND_Attenuation1.SND_Attenuation1" null null))))
                  (:`then_1`
                    (`GameplayStatics.PlaySoundAtLocation` "/Game/Audio/SndFX/keyholeTurn.keyholeTurn" (`SceneComponent.K2_GetComponentLocation` _closetkey) (struct) 1.0 1.0 0.0 "/Game/Audio/SND_Attenuation1.SND_Attenuation1" null null))))
              (:`then_1`
                (`GameplayStatics.PlaySoundAtLocation` "/Game/Audio/SndFX/keyholeInsert.keyholeInsert" (`SceneComponent.K2_GetComponentLocation` _closetkey) (struct) 1.0 1.0 0.0 "/Game/Audio/SND_Attenuation1.SND_Attenuation1" null null)))))))))

(fn `UserConstructionScript`
  (`SceneComponent.SetVisibility` (`self.wirecutter`) false false)
  (`SceneComponent.SetVisibility` (`self.ClosetKey`) false false))