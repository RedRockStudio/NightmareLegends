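; BP_SafeInWall is a two-stage quest puzzle: a wall safe revealed behind a sliding picture.
; Box overlaps show empty-handed players stage-based tips and detect tagged QuestObj1 items.
; The picture piece slides the picture aside; the handle then opens the safe, using delayed MoveComponentTo animations and sounds.
; Each accepted item reveals a hidden mesh and destroys the player's UnderAimActor, not the overlapping actor directly.
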(event `self.Box.OnComponentBeginOverlap`
  (params (OverlappedComponent :type "PrimitiveComponent Object Reference") (OtherActor :type "Actor Object Reference") (OtherComp :type "PrimitiveComponent Object Reference") (OtherBodyIndex :type Integer) (bFromSweep :type Boolean) (SweepResult :type "HitResult Structure (by ref)"))
  (`|ExecutionSequence`
    (:`then_0`
      ;[0.2102 0.3762 0.651] Tips
      (bind _asfirst_person_character (cast `/Game/FirstPersonBP/Blueprints/FirstPersonCharacter` OtherActor))
      (if (and (`/Game/FirstPersonBP/Blueprints/FirstPersonCharacter.IsHandEmpty?` _asfirst_person_character) (not (`self.QuestDone`)))
        (if (`self.PicMoved`)
          (bind _mainwidget (`/Game/FirstPersonBP/Blueprints/FirstPersonCharacter.MainWidget` _asfirst_person_character))
          (set `/Game/Widgets/MainWidget.CurrTipName` "Picture2" _mainwidget)
          (`/Game/Widgets/MainWidget.Tips` _mainwidget)
          (else
            (set `/Game/Widgets/MainWidget.CurrTipName` "Picture1" _mainwidget)
            (`/Game/Widgets/MainWidget.Tips` _mainwidget)))))
    (:`then_1`
      (bind _asquest_obj_1 (cast `/Game/Blueprints/QuestObj/QuestObj1` OtherActor))
      (`|ExecutionSequence`
        (:`then_0`
          (if (`self.ActorHasTag` _asquest_obj_1 "QO_PicPiece")
            (set `self.PicMoved` true)
            (bind _asquest_obj_1_2 (cast `/Game/Blueprints/QuestObj/QuestObj1` (`/Game/FirstPersonBP/Blueprints/FirstPersonCharacter.UnderAimActor` (cast `/Game/FirstPersonBP/Blueprints/FirstPersonCharacter` (`GameplayStatics.GetPlayerPawn` 0) :!pure true))))
            (`self.K2_DestroyActor` _asquest_obj_1_2)
            (`GameplayStatics.PlaySoundAtLocation` "/Game/Audio/SndFX/takeFabricObj.takeFabricObj" (`SceneComponent.K2_GetComponentLocation` (`self.SafeMesh`)) (struct) 1.0 1.0 0.0 "/Game/Audio/SND_Attenuation1.SND_Attenuation1" null null)
            (`SceneComponent.SetVisibility` (`self.PicQuestPiece`) true false)
            (`KismetSystemLibrary.Delay` 1.5)
            (`GameplayStatics.PlaySoundAtLocation` "/Game/Audio/SndFX/PicSliding.PicSliding" (`SceneComponent.K2_GetComponentLocation` (`self.SafeMesh`)) (struct) 1.0 1.0 0.0 "/Game/Audio/SND_Attenuation1.SND_Attenuation1" null null)
            (`KismetSystemLibrary.MoveComponentTo` (`self.Pic`) (70.0 22.0 15.0) (struct) true true 1.0)))
        (:`then_1`
          (if (and (`self.ActorHasTag` _asquest_obj_1 "QO_SafeHandle") (`self.PicMoved`))
            (set `self.QuestDone` true)
            (bind _asquest_obj_1_3 (cast `/Game/Blueprints/QuestObj/QuestObj1` (`/Game/FirstPersonBP/Blueprints/FirstPersonCharacter.UnderAimActor` (cast `/Game/FirstPersonBP/Blueprints/FirstPersonCharacter` (`GameplayStatics.GetPlayerPawn` 0) :!pure true))))
            (`self.K2_DestroyActor` _asquest_obj_1_3)
            (`GameplayStatics.PlaySoundAtLocation` "/Game/Audio/SndFX/takeMetObj.takeMetObj" (`SceneComponent.K2_GetComponentLocation` (`self.SafeMesh`)) (struct) 1.0 1.0 0.0 "/Game/Audio/SND_Attenuation1.SND_Attenuation1" null null)
            (`SceneComponent.SetVisibility` (`self.DoorHandleMesh`) true false)
            (`KismetSystemLibrary.Delay` 0.5)
            (`GameplayStatics.PlaySoundAtLocation` "/Game/Audio/SndFX/bookFlip2.bookFlip2" (`SceneComponent.K2_GetComponentLocation` (`self.SafeMesh`)) (struct) 1.0 1.0 0.0 "/Game/Audio/SND_Attenuation1.SND_Attenuation1" null null)
            (`KismetSystemLibrary.MoveComponentTo` (`self.DoorHandleMesh`) (-16.740444 2.065805 0.112751) (struct :`Pitch` -80.0) true true 1.0)
            (`KismetSystemLibrary.Delay` 0.5)
            (`GameplayStatics.PlaySoundAtLocation` "/Game/Audio/SndFX/bookFlip2.bookFlip2" (`SceneComponent.K2_GetComponentLocation` (`self.SafeMesh`)) (struct) 1.0 1.0 0.0 "/Game/Audio/SND_Attenuation1.SND_Attenuation1" null null)
            (`KismetSystemLibrary.MoveComponentTo` (`self.DoorMesh`) (26.061447 15.604416 20.344395) (struct :`Yaw` -100.0) true true 1.0)))))))

(fn `UserConstructionScript`
  (`SceneComponent.SetVisibility` (`self.PicQuestPiece`) false false)
  (`SceneComponent.SetVisibility` (`self.DoorHandleMesh`) false false))